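; Player-placeable zombie-defence turret that fires sphere traces, damaging BP_ZombieMaster targets with muzzle and impact effects.
; Ammo doubles as health: each shot damages the turret itself, and at zero it tilts down, shows a reload widget, then rises refilled after a timer.
; Timelines and a looping timer spin the barrel up and down.
; Interacting with a live turret hands its stats to the player's drop system and destroys it for re-placement.
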(event `self.ReceiveAnyDamage`
  (params (Damage :type "Float (single-precision)") (DamageType :type "DamageType Object Reference") (InstigatedBy :type "Controller Object Reference") (DamageCauser :type "Actor Object Reference"))
  ;[0.1146 0.1146 0.1146] Event Any Damage
  (if (not (`self.IsDeath?`))
    (set `self.Ammo` (- (`self.Ammo`) Damage))
    (if (<= (`self.Ammo`) 0.0)
      (set `self.IsDeath?` true)
      (`self.DeathTurret`)
      (`self.DeathTimer`))))

(event `self.ReceiveBeginPlay`
  ;[1 1 1] Begin play Ref Xidget
  (bind _asbp_player (cast `/Game/Assets/Blueprint/Player/BP_Player` (`GameplayStatics.GetPlayerCharacter` 0)))
  (set `self.As BP Player` _asbp_player)
  (bind _aswbp_reload_turret (cast `/Game/BATET/Widget/WBP_ReloadTurret` (`WidgetComponent.GetUserWidgetObject` (`self.Widget`))))
  (set `/Game/BATET/Widget/WBP_ReloadTurret.Bp_TurretRef` self _aswbp_reload_turret)
  ;;[1 1 1] Set atk Count to atk speed
  (set `self.SpeedAttackCount` (`self.SpeedAttack`)))

(event `/Game/BlueprintCommun/BPI_Interact.Interact`
  (params (PlayerRef :type "/Game/Assets/Blueprint/Player/BP_Player Object Reference"))
  (bind _bpc_dropsystem (`/Game/Assets/Blueprint/Player/BP_Player.BPC_DropSystem` PlayerRef))
  ;[1 1 1] Save Variable pickup turret
  (if (and (not (`self.IsDeath?`)) (`/Game/BATET/Bp_BuildTurret/BPC_DropSystemTurret.IsPosed?` _bpc_dropsystem))
    (set `/Game/BATET/Bp_BuildTurret/BPC_DropSystemTurret.IsPosed?` false _bpc_dropsystem)
    (`UserWidget.AddToViewport` (`/Game/BATET/Bp_BuildTurret/BPC_DropSystemTurret.WidgetTurretDrop` _bpc_dropsystem) 0)
    (set `/Game/BATET/Bp_BuildTurret/BPC_DropSystemTurret.In drop mode ?` true _bpc_dropsystem)
    (set `/Game/BATET/Bp_BuildTurret/BPC_DropSystemTurret.AmoCurrentTurret` (`self.Ammo`) _bpc_dropsystem)
    (set `/Game/BATET/Bp_BuildTurret/BPC_DropSystemTurret.DistanceTurret` (`self.DistanceShoot`) _bpc_dropsystem)
    (set `/Game/BATET/Bp_BuildTurret/BPC_DropSystemTurret.Death?` (`self.IsDeath?`) _bpc_dropsystem)
    (set `/Game/BATET/Bp_BuildTurret/BPC_DropSystemTurret.SpeedAtk` (`self.SpeedAttack`) _bpc_dropsystem)
    (set `/Game/BATET/Bp_BuildTurret/BPC_DropSystemTurret.TimeToReload` (`self.TimeToReload`) _bpc_dropsystem)
    (`self.K2_DestroyActor`)))

(event `DeathTimer`
  ;[1 1 1] Timer Reload
  (bind _returnvalue (`KismetSystemLibrary.K2_SetTimerDelegate` (delegate `Timer`) (`self.TimeToReload`)))
  (set `self.TimerRealod` _returnvalue)
  (`SceneComponent.SetVisibility` (`self.Widget`) true false)
  (`GameplayStatics.PlaySoundAtLocation` "/Game/CHARONNAT/SoundDesign/Sounds/Weapons/Turret/A_TurretDeath_Cue.A_TurretDeath_Cue" (`self.K2_GetActorLocation`) (struct) 1.0 1.0 0.0 null null null null))

(event `RotateBar`
  ;[1 1 1] Timer Reload
  (`SceneComponent.K2_SetRelativeRotation` (`self.Widget`) (`KismetMathLibrary.FindLookAtRotation` (`SceneComponent.K2_GetComponentLocation` (`self.Widget`)) (`self.K2_GetActorLocation` (`self.As BP Player`))) false false))

(event `Timer`
  ;[1 1 1] Timer Reload
  (`self.RealodEnd`)
  (`SceneComponent.SetVisibility` (`self.Widget`) false false)
  (`KismetSystemLibrary.K2_ClearAndInvalidateTimerHandle` (`self.TimerRotate`))
  (`GameplayStatics.PlaySoundAtLocation` "/Game/CHARONNAT/SoundDesign/Sounds/Weapons/Turret/A_TurretReload_Cue.A_TurretReload_Cue" (`self.K2_GetActorLocation`) (struct) 1.0 1.0 0.0 null null null null))

(event `StartShoot`
  ;[1 1 1] Loop rotate turret
  (bind _returnvalue (`KismetSystemLibrary.K2_SetTimerDelegate` (delegate `RotateCanon`) (`GameplayStatics.GetWorldDeltaSeconds`) true))
  (set `self.TimerRotateCanonRef` _returnvalue)
  (`GameplayStatics.PlaySoundAtLocation` "/Game/CHARONNAT/SoundDesign/Sounds/Weapons/Turret/A_Turret_Cue.A_Turret_Cue" (`self.K2_GetActorLocation`) (struct) 1.0 1.0 0.0 null null null null))

(event `BeginShoot`
  ;[1 1 1] Begin, End Rotate Turret
  (set `self.Begin?` true)
  (bind (_direction _rotate) (`Timeline|RotateBegin` :!label _label)
    (:`Update`
      (`SceneComponent.K2_AddRelativeRotation` (`self.Canon`) (`KismetMathLibrary.MakeRotator` (* _rotate (`self.TurnSpeedTurret`))) false false))
    (:`Finished`
      (if (`self.Begin?`)
        (`self.StartShoot`)))))

(event `RotateCanon`
  ;[1 1 1] Loop rotate turret
  (`SceneComponent.K2_AddRelativeRotation` (`self.Canon`) (`KismetMathLibrary.MakeRotator` (+ (`self.TurnSpeedTurret`) 1.0)) false false))

(event `EndShoot`
  ;[1 1 1] Begin, End Rotate Turret
  (`KismetSystemLibrary.K2_ClearAndInvalidateTimerHandle` (`self.TimerRotateCanonRef`))
  (set `self.Begin?` false)
  (goto _label :!via `Reverse`))

(event `DeathTurret`
  (bind (_relativerotation_roll _relativerotation_pitch _relativerotation_yaw) (`KismetMathLibrary.BreakRotator` (`SceneComponent.RelativeRotation` (`self.TurretTopNoCanon`))))
  ;[1 1 1] No amo Down / Up Turret
  (bind (_direction _blend) (`Timeline|BlendDeath` :!via `PlayFromStart` :!label _label_2)
    (:`Update`
      (`SceneComponent.K2_SetRelativeRotation` (`self.TurretTopNoCanon`) (`KismetMathLibrary.MakeRotator` _relativerotation_roll (`KismetMathLibrary.Lerp` 0.0 -30.0 _blend) _relativerotation_yaw) false false))
    (:`Finished`
      (if (`self.EndRealod?`)
        (set `self.IsDeath?` false)
        (set `self.Ammo` 100.0)
        (set `self.EndRealod?` false)))))

(event `RealodEnd`
  ;[1 1 1] No amo Down / Up Turret
  (set `self.EndRealod?` true)
  (goto _label_2 :!via `ReverseFromEnd`))

(fn `LineTraceShoot`
  (bind _canon (`self.Canon`))
  (bind _returnvalue (`SceneComponent.K2_GetComponentLocation` _canon))
  (bind (_outhit _returnvalue_2) (`KismetSystemLibrary.SphereTraceSingle` _returnvalue (+ _returnvalue (* (`SceneComponent.GetForwardVector` _canon) (`self.DistanceShoot`))) 5.0 "TraceTypeQuery1"))
  (`GameplayStatics.ApplyDamage` self 1.0)
  (`NiagaraFunctionLibrary.SpawnSystemAtLocation` "/Game/Assets/Niagara/Gun_VFX/Niagara_FX/Muzzle_Flashes/NS_Sniper_Muzzle_flashes_02.NS_Sniper_Muzzle_flashes_02" (`SceneComponent.K2_GetComponentLocation` (`self.Arrow`)))
  (if _returnvalue_2
    (bind (_bblockinghit _binitialoverlap _time _distance _location _impactpoint _normal _impactnormal _physmat _hitactor) (`GameplayStatics.BreakHitResult` _outhit))
    (bind _asbp_zombie_master (cast `/Game/Broquere/Zombie/Master/BP_ZombieMaster` _hitactor))
    (bind _output_get (set `self.As BP Zombie Master` _asbp_zombie_master))
    (`GameplayStatics.ApplyDamage` _output_get (`self.Base Damage`))
    (`NiagaraFunctionLibrary.SpawnSystemAtLocation` "/Game/YI_BloodDroplets/Particles/GPU/FX_EntranceWound_Rifle_GPU.FX_EntranceWound_Rifle_GPU" _impactpoint)))

(fn `UserConstructionScript`)