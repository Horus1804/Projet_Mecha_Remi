(event `self.ReceiveBeginPlay`
  (bind _returnvalue (`GameplayStatics.GetPlayerController` 0))
  ;[0.01938 0.01938 0.01938] Event begin play PlayerRef Et Add Input
  (`/Engine/EditorBlueprintResources/StandardMacros.IsValid` _returnvalue
    (:`Is Valid`
      (`EnhancedInputSubsystemInterface.AddMappingContext` (pcsubsystem `EnhancedInputLocalPlayerSubsystem` _returnvalue) "/Game/Assets/Blueprint/Input/IMC_Utility.IMC_Utility" 0 (struct))
      (bind _asbp_player (cast `/Game/Assets/Blueprint/Player/BP_Player` (`GameplayStatics.GetPlayerCharacter` 0)))
      (set `self.As BP PlayerRef` _asbp_player)
      (set `self.CameraPlayerRef` (`/Game/Assets/Blueprint/Player/BP_Player.Camera` _asbp_player))
      (bind _returnvalue_2 (`|CreateWidget` "/Game/BATET/Widget/WBP_TurretDropMode.WBP_TurretDropMode_C"))
      (set `self.WidgetTurretDrop` _returnvalue_2))))

(event `EnhancedInput|/Game/Assets/Blueprint/Input/Input/IA_BuildTurret`
  (params (ActionValue :type Boolean) (ElapsedSeconds :type "Float (double-precision)") (TriggeredSeconds :type "Float (double-precision)") (InputAction :type "InputAction Object Reference" :default "/Game/Assets/Blueprint/Input/Input/IA_BuildTurret.IA_BuildTurret"))
  ;[0.01938 0.01938 0.01938] Active / Deactive Drop mode
  (:`Started`
    (if (and (not (`self.In drop mode ?`)) (not (`self.IsPosed?`)))
      (set `self.In drop mode ?` true)
      (`UserWidget.AddToViewport` (`self.WidgetTurretDrop`) 0)
      (set `/Game/Assets/Blueprint/Player/BP_Player.CanFire` false (`self.As BP PlayerRef`))
      (else
        (set `self.In drop mode ?` false :!label _label)
        (bind _previewmesh (`self.PreviewMesh`)
          (:`then`
            (`StaticMeshComponent.SetStaticMesh` _previewmesh null)
            (set `self.PreviewMesh` null)
            (`self.Reset Drop Mode`)
            (`Widget.RemoveFromParent` (`self.WidgetTurretDrop`))
            (set `/Game/Assets/Blueprint/Player/BP_Player.CanFire` true (`self.As BP PlayerRef`)))
          (:`else`))))))

(event `EnhancedInput|/Game/Assets/Blueprint/Input/Input/IA_Drone`
  (params (ActionValue :type Boolean) (ElapsedSeconds :type "Float (double-precision)") (TriggeredSeconds :type "Float (double-precision)") (InputAction :type "InputAction Object Reference" :default "/Game/Assets/Blueprint/Input/Input/IA_Drone.IA_Drone"))
  (bind _returnvalue (`KismetMathLibrary.RandomFloatInRange` -100.0 100.0))
  (bind (_returnvalue_x _returnvalue_y _returnvalue_z) (`KismetMathLibrary.BreakVector` (`Actor.K2_GetActorLocation` (`self.As BP PlayerRef`))))
  (:`Started`
    (if (`self.PosedDrone?`)
      (set `self.PosedDrone?` false)
      (bind _refdrone (`self.RefDrone`)
        (:`then`
          (`Actor.K2_DestroyActor` _refdrone))
        (:`else`
          (`KismetSystemLibrary.PrintString` "No")))
      (else
        (set `self.PosedDrone?` true)
        (bind _returnvalue_2 (`AIBlueprintHelperLibrary.SpawnAIFromClass` "/Game/BATET/Drone/Bp_Drone.Bp_Drone_C" "/Game/BATET/Drone/BT_Drone.BT_Drone" (`KismetMathLibrary.MakeVector` (+ _returnvalue_x _returnvalue) (+ _returnvalue_y _returnvalue) (+ _returnvalue_z 130.0)) (struct) true null))
        (bind _output_get (set `self.RefDrone` _returnvalue_2))
        (`KismetSystemLibrary.PrintString` (`KismetSystemLibrary.GetDisplayName` _output_get))))))

(event `Stop Drop Mode`
  ;[0.01938 0.01938 0.01938] Active / Deactive Drop mode
  (goto _label))

(event `self.ReceiveTick`
  (params (DeltaSeconds :type "Float (single-precision)"))
  ;[0.01938 0.01938 0.01938] Event Tick Preview Mesh
  (`|ExecutionSequence`
    (:`then_0`
      (if (`self.In drop mode ?`)
        (`self.PreviewLoop`)))))

(event `Reset Drop Mode`
  (bind _previewmesh (`self.PreviewMesh`))
  ;[0.01938 0.01938 0.01938] Line Trace Preview Mesh
  (goto _label_2 :!via `Reset`))

(event `PreviewLoop`
  (bind _previewmesh (`self.PreviewMesh`))
  (bind (_returnvalue_location _returnvalue_rotation) (`KismetMathLibrary.BreakTransform` (`SceneComponent.K2_GetComponentToWorld` (`self.CameraPlayerRef`))))
  ;[0.01938 0.01938 0.01938] Line Trace Preview Mesh
  (bind (_outhit _returnvalue) (`KismetSystemLibrary.LineTraceSingle` _returnvalue_location (+ _returnvalue_location (* (`KismetMathLibrary.GetForwardVector` _returnvalue_rotation) (`self.DistanceToDrop`))) "TraceTypeQuery1"))
  (if _returnvalue
    (set `self.CanDrop?` true)
    (`|ExecutionSequence`
      (:`then_0`
        (`/Engine/EditorBlueprintResources/StandardMacros.DoOnce` false :!label _label_2
          (:`Completed`
            (bind _returnvalue_2 (`|AddComponentByClass` (`self.As BP PlayerRef`) "/Script/Engine.StaticMeshComponent" false (`self.Drop Preview Transform`)))
            (bind _output_get (set `self.PreviewMesh` _returnvalue_2))
            (`StaticMeshComponent.SetStaticMesh` _output_get "/Game/BATET/Asset/Touret/SM_FullTurret.SM_FullTurret")
            (`PrimitiveComponent.SetMaterial` _previewmesh 0 "/Game/BATET/Asset/Touret/M_Preview.M_Preview")
            (`PrimitiveComponent.SetCollisionEnabled` _previewmesh "NoCollision"))))
      (:`then_1`
        (bind (_bblockinghit _binitialoverlap _time _distance _location _impactpoint _normal _impactnormal _physmat _hitactor) (`GameplayStatics.BreakHitResult` _outhit))
        (bind (_returnvalue_roll _returnvalue_pitch _returnvalue_yaw) (`KismetMathLibrary.BreakRotator` (`KismetMathLibrary.FindLookAtRotation` (`Actor.K2_GetActorLocation` (`self.As BP PlayerRef`)) _location)))
        (bind _output_get_2 (set `self.Drop Preview Transform` (`KismetMathLibrary.MakeTransform` _location (`KismetMathLibrary.MakeRotator` 0.0 0.0 _returnvalue_yaw) (0.01 0.01 0.01))))
        (`SceneComponent.K2_SetWorldTransform` (`self.PreviewMesh`) _output_get_2 false false)))))

(event `EnhancedInput|/Game/Assets/Blueprint/Input/Input/IA_Fire`
  (params (ActionValue :type Boolean) (ElapsedSeconds :type "Float (double-precision)") (TriggeredSeconds :type "Float (double-precision)") (InputAction :type "InputAction Object Reference" :default "/Game/Assets/Blueprint/Input/Input/IA_Fire.IA_Fire"))
  (bind (_drop_preview_transform_location _drop_preview_transform_rotation) (`KismetMathLibrary.BreakTransform` (`self.Drop Preview Transform`)))
  ;[0.01938 0.01938 0.01938] Place Actor
  (:`Started`
    (if (and (`self.In drop mode ?`) (`self.CanDrop?`) (not (`self.IsPosed?`)))
      (bind _returnvalue (`AIBlueprintHelperLibrary.SpawnAIFromClass` "/Game/BATET/Turret/Bp_Turret.Bp_Turret_C" "/Game/BATET/Turret/BT_Turret.BT_Turret" _drop_preview_transform_location _drop_preview_transform_rotation true null))
      (bind _asbp_turret (cast `/Game/BATET/Turret/Bp_Turret` _returnvalue))
      (bind _output_get (set `self.As Bp Turret` _asbp_turret))
      (set `/Game/BATET/Turret/Bp_Turret.DistanceShoot` (`self.DistanceTurret`) _output_get)
      (set `/Game/BATET/Turret/Bp_Turret.Ammo` (`self.AmoCurrentTurret`) _output_get)
      (set `/Game/BATET/Turret/Bp_Turret.IsDeath?` (`self.Death?`) _output_get)
      (set `/Game/BATET/Turret/Bp_Turret.SpeedAttack` (`self.SpeedAtk`) _output_get)
      (set `/Game/BATET/Turret/Bp_Turret.TimeToReload` (`self.TimeToReload`) _output_get)
      (set `self.IsPosed?` true)
      (`self.Stop Drop Mode`))))