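; BPC_BuyItem is a Blueprint that detects what the player looks at and toggles that actor's UI message, presumably for buying items.
; It caches the BP_Player character on BeginPlay, then every Tick sphere-traces a short distance forward from its camera.
; A hit actor is stored and sent AffUiMessage; when nothing is hit, the last stored actor gets StopUiMessage, so switching directly between actors skips the stop.
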(event `self.ReceiveBeginPlay`
  (bind _asbp_player (cast `/Game/Assets/Blueprint/Player/BP_Player` (`GameplayStatics.GetPlayerCharacter` 0)))
  (set `self.As BP Player` _asbp_player))

(event `self.ReceiveTick`
  (params (DeltaSeconds :type "Float (single-precision)"))
  (bind _camera (`/Game/Assets/Blueprint/Player/BP_Player.Camera` (`self.As BP Player`)))
  (bind _returnvalue (`SceneComponent.K2_GetComponentLocation` _camera))
  (bind (_outhit _returnvalue_2) (`KismetSystemLibrary.SphereTraceSingle` :`Start` _returnvalue :`End` (+ _returnvalue (* (`SceneComponent.GetForwardVector` _camera) 200.0)) :`Radius` 20.0 :`TraceChannel` "TraceTypeQuery3" :`DrawTime` 0.0))
  (if _returnvalue_2
    (bind _output_get (set `self.Hit Actor` (`.HitActor` (`GameplayStatics.BreakHitResult` _outhit))))
    (message `/Game/BATET/Bp_buyitem/BPI_AffUI.AffUi` _output_get (`self.As BP Player`))
    (else
      (bind _hit_actor (`self.Hit Actor`)
        (:`then`
          (message `/Game/BATET/Bp_buyitem/BPI_AffUI.StopUi` _hit_actor (`self.As BP Player`)))
        (:`else`)))))