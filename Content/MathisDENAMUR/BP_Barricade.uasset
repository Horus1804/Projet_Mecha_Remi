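; Five-plank zombie barricade that zombies tear down and the player rebuilds for score and money.
; PlankIndex tracks standing planks: zombie damage moves the top one to its spline's endpoint, while Interact restores one with a small reward.
; Losing the last plank opens the Block collision except on GameTraceChannel1, and restoring the first closes it again.
; InstantRebuild quickly restores all five planks and grants a larger reward.
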(event `self.ReceiveAnyDamage`
  (params (Damage :type "Float (single-precision)") (DamageType :type "DamageType Object Reference") (InstigatedBy :type "Controller Object Reference") (DamageCauser :type "Actor Object Reference"))
  (bind _spline_3 (`self.Spline 3`))
  (bind _spline_4 (`self.Spline 4`))
  (bind _spline_5 (`self.Spline 5`))
  (bind _spline_2 (`self.Spline 2`))
  (bind _spline_1 (`self.Spline 1`))
  (cast `/Game/Broquere/Zombie/Master/BP_ZombieMaster` DamageCauser)
  (switch `int` (`self.PlankIndex`)
    (:`1`
      (`KismetSystemLibrary.MoveComponentTo` (`self.Plank 1`) (`SplineComponent.GetLocationAtDistanceAlongSpline` _spline_1 (`SplineComponent.GetSplineLength` _spline_1) "Local"))
      (set `self.PlankIndex` 0)
      (`PrimitiveComponent.SetCollisionResponseToAllChannels` (`self.Block`) "ECR_Ignore")
      (`PrimitiveComponent.SetCollisionResponseToChannel` (`self.Block`) "ECC_GameTraceChannel1" "ECR_Block")
      (`PrimitiveComponent.SetCollisionResponseToChannel` (`self.Block`) "ECC_GameTraceChannel1" "ECR_Block")
      (`GameplayStatics.PlaySoundAtLocation` "/Game/CHARONNAT/SoundDesign/Sounds/Player/Barricades/A_BarricadesDestroy-001_Cue.A_BarricadesDestroy-001_Cue" (`self.K2_GetActorLocation`) (struct) 1.0 1.0 0.0 "/Game/YI_ModularZombies/Sounds/Master/SA_Low.SA_Low" null null null))
    (:`2`
      (`KismetSystemLibrary.MoveComponentTo` (`self.Plank 2`) (`SplineComponent.GetLocationAtDistanceAlongSpline` _spline_2 (`SplineComponent.GetSplineLength` _spline_2) "Local") (struct :`Yaw` 64.0))
      (set `self.PlankIndex` 1)
      (`GameplayStatics.PlaySoundAtLocation` "/Game/CHARONNAT/SoundDesign/Sounds/Player/Barricades/A_BarricadesDestroy-001_Cue.A_BarricadesDestroy-001_Cue" (`self.K2_GetActorLocation`) (struct) 1.0 1.0 0.0 "/Game/YI_ModularZombies/Sounds/Master/SA_Low.SA_Low" null null null))
    (:`3`
      (`KismetSystemLibrary.MoveComponentTo` (`self.Plank 3`) (`SplineComponent.GetLocationAtDistanceAlongSpline` _spline_3 (`SplineComponent.GetSplineLength` _spline_3) "Local") (struct :`Yaw` -34.0))
      (set `self.PlankIndex` 2)
      (`GameplayStatics.PlaySoundAtLocation` "/Game/CHARONNAT/SoundDesign/Sounds/Player/Barricades/A_BarricadesDestroy-001_Cue.A_BarricadesDestroy-001_Cue" (`self.K2_GetActorLocation`) (struct) 1.0 1.0 0.0 "/Game/YI_ModularZombies/Sounds/Master/SA_Low.SA_Low" null null null))
    (:`4`
      (`KismetSystemLibrary.MoveComponentTo` (`self.Plank 4`) (`SplineComponent.GetLocationAtDistanceAlongSpline` _spline_4 (`SplineComponent.GetSplineLength` _spline_4) "Local") (struct :`Yaw` 45.0))
      (set `self.PlankIndex` 3)
      (`GameplayStatics.PlaySoundAtLocation` "/Game/CHARONNAT/SoundDesign/Sounds/Player/Barricades/A_BarricadesDestroy-001_Cue.A_BarricadesDestroy-001_Cue" (`self.K2_GetActorLocation`) (struct) 1.0 1.0 0.0 "/Game/YI_ModularZombies/Sounds/Master/SA_Low.SA_Low" null null null))
    (:`5`
      (`KismetSystemLibrary.MoveComponentTo` (`self.Plank 5`) (`SplineComponent.GetLocationAtDistanceAlongSpline` _spline_5 (`SplineComponent.GetSplineLength` _spline_5) "Local") (struct :`Yaw` 26.0))
      (set `self.PlankIndex` 4)
      (`GameplayStatics.PlaySoundAtLocation` "/Game/CHARONNAT/SoundDesign/Sounds/Player/Barricades/A_BarricadesDestroy-001_Cue.A_BarricadesDestroy-001_Cue" (`self.K2_GetActorLocation`) (struct) 1.0 1.0 0.0 "/Game/YI_ModularZombies/Sounds/Master/SA_Low.SA_Low" null null null))))

(event `self.ReceiveBeginPlay`
  (set `self.As BP Player` (cast `/Game/Assets/Blueprint/Player/BP_Player` (`GameplayStatics.GetPlayerCharacter` 0) :!pure true)))

(event `/Game/BlueprintCommun/BPI_Interact.Interact`
  (params (PlayerRef :type "/Game/Assets/Blueprint/Player/BP_Player Object Reference"))
  (bind _as_bp_player (`self.As BP Player`))
  (switch `int` (`self.PlankIndex`)
    (:`0`
      (`KismetSystemLibrary.MoveComponentTo` (`self.Plank 1`) (0.0 0.0 0.0) (struct :`Pitch` 10.0 :`Roll` 90.0))
      (set `self.PlankIndex` 1)
      (`PrimitiveComponent.SetCollisionResponseToAllChannels` (`self.Block`) "ECR_Block")
      (`GameplayStatics.PlaySound2D` "/Game/CHARONNAT/SoundDesign/Sounds/Player/Barricades/A_BarricadeHammer_ZA01_27_Cue.A_BarricadeHammer_ZA01_27_Cue" 1.0 1.0 0.0 null null))
    (:`1`
      (`KismetSystemLibrary.MoveComponentTo` (`self.Plank 2`) (0.0 0.0 0.0) (struct :`Roll` 90.0))
      (set `self.PlankIndex` 2)
      (`GameplayStatics.PlaySound2D` "/Game/CHARONNAT/SoundDesign/Sounds/Player/Barricades/A_BarricadeHammer_ZA01_27_Cue.A_BarricadeHammer_ZA01_27_Cue" 1.0 1.0 0.0 null null))
    (:`2`
      (`KismetSystemLibrary.MoveComponentTo` (`self.Plank 3`) (0.0 -5.0 0.0) (struct :`Pitch` 180.0 :`Roll` 90.0))
      (set `self.PlankIndex` 3)
      (`GameplayStatics.PlaySound2D` "/Game/CHARONNAT/SoundDesign/Sounds/Player/Barricades/A_BarricadeHammer_ZA01_27_Cue.A_BarricadeHammer_ZA01_27_Cue" 1.0 1.0 0.0 null null))
    (:`3`
      (`KismetSystemLibrary.MoveComponentTo` (`self.Plank 4`) (0.0 -5.0 0.0) (struct :`Pitch` -90.0 :`Roll` 90.0))
      (set `self.PlankIndex` 4)
      (`GameplayStatics.PlaySound2D` "/Game/CHARONNAT/SoundDesign/Sounds/Player/Barricades/A_BarricadeHammer_ZA01_27_Cue.A_BarricadeHammer_ZA01_27_Cue" 1.0 1.0 0.0 null null))
    (:`4`
      (`KismetSystemLibrary.MoveComponentTo` (`self.Plank 5`) (0.0 -5.0 0.0) (struct :`Pitch` 90.0 :`Roll` 90.0))
      (set `self.PlankIndex` 5)
      (`GameplayStatics.PlaySound2D` "/Game/CHARONNAT/SoundDesign/Sounds/Player/Barricades/A_BarricadeHammer_ZA01_27_Cue.A_BarricadeHammer_ZA01_27_Cue" 1.0 1.0 0.0 null null)))
  (`/Game/Assets/Blueprint/Player/BP_Player.SetScore` _as_bp_player (+ (`/Game/Assets/Blueprint/Player/BP_Player.Score` _as_bp_player) 10))
  (`/Game/Assets/Blueprint/Player/BP_Player.SetMoney` _as_bp_player (+ (`/Game/Assets/Blueprint/Player/BP_Player.Money` _as_bp_player) 10)))

(event `InstantRebuild`
  (bind _as_bp_player (`self.As BP Player`))
  (`GameplayStatics.PlaySoundAtLocation` "/Game/CHARONNAT/SoundDesign/Sounds/Player/Barricades/A_BarricadesDestroy-001_Cue.A_BarricadesDestroy-001_Cue" (`self.K2_GetActorLocation`) (struct) 1.0 1.0 0.0 "/Game/YI_ModularZombies/Sounds/Master/SA_Low.SA_Low" null null null)
  (`PrimitiveComponent.SetCollisionResponseToAllChannels` (`self.Block`) "ECR_Block")
  (`KismetSystemLibrary.MoveComponentTo` (`self.Plank 1`) (0.0 0.0 0.0) (struct :`Pitch` 10.0 :`Roll` 90.0) false false 0.05)
  (`KismetSystemLibrary.MoveComponentTo` (`self.Plank 2`) (0.0 0.0 0.0) (struct :`Roll` 90.0) false false 0.05)
  (`KismetSystemLibrary.MoveComponentTo` (`self.Plank 3`) (0.0 -5.0 0.0) (struct :`Pitch` 180.0 :`Roll` 90.0) false false 0.05)
  (`KismetSystemLibrary.MoveComponentTo` (`self.Plank 4`) (0.0 -5.0 0.0) (struct :`Pitch` -90.0 :`Roll` 90.0) false false 0.05)
  (`KismetSystemLibrary.MoveComponentTo` (`self.Plank 5`) (0.0 -5.0 0.0) (struct :`Pitch` 90.0 :`Roll` 90.0) false false 0.05)
  (`PrimitiveComponent.SetCollisionResponseToAllChannels` (`self.Block`) "ECR_Block")
  (set `self.PlankIndex` 5)
  (`/Game/Assets/Blueprint/Player/BP_Player.SetScore` _as_bp_player (+ (`/Game/Assets/Blueprint/Player/BP_Player.Score` _as_bp_player) 50))
  (`/Game/Assets/Blueprint/Player/BP_Player.SetMoney` _as_bp_player (+ (`/Game/Assets/Blueprint/Player/BP_Player.Money` _as_bp_player) 50)))

(fn `UserConstructionScript`)