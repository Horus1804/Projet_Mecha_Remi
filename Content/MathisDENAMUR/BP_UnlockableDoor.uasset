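; Purchasable door that the player unlocks with money, swinging its panels open through a timeline.
; Interact charges the player, raises the cost of every door in the level and also opens a linked door when flagged.
; AffUi and StopUi toggle the lock prompt widget and pass it the player reference.
; The construction script sets frame and panel meshes for an optional double-door variant.
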(event `self.ReceiveBeginPlay`
  (bind _aswbp_lock_door (cast `/Game/BATET/Widget/WBP_LockDoor` (`WidgetComponent.GetUserWidgetObject` (`self.LockDoor`))))
  (bind _output_get (set `self.As WBP Lock Door` _aswbp_lock_door))
  (set `/Game/BATET/Widget/WBP_LockDoor.DoorRef` self _output_get)
  (set `self.As BP Player` (cast `/Game/Assets/Blueprint/Player/BP_Player` (`GameplayStatics.GetPlayerCharacter` 0) :!pure true))
  (bind _outactors (`GameplayStatics.GetAllActorsOfClass` "BP_UnlockableDoor_C"))
  (set `self.All Doors` _outactors))

(event `open`
  (bind (_direction _open) (`Timeline|Open door` :!label _label)
    (:`Update`
      (`PrimitiveComponent.SetCollisionEnabled` (`self.Door 1`) "NoCollision")
      (`PrimitiveComponent.SetCollisionEnabled` (`self.Door 2`) "NoCollision")
      (bind _returnvalue (* _open -90.0))
      (`SceneComponent.K2_SetRelativeRotation` (`self.Door 1`) (`KismetMathLibrary.MakeRotator` 0.0 0.0 _returnvalue) false false)
      (`SceneComponent.K2_SetRelativeRotation` (`self.Door 2`) (`KismetMathLibrary.MakeRotator` 0.0 0.0 (* _returnvalue -1.0)) false false))
    (:`Finished`
      (set `self.Is open` true)
      (`PrimitiveComponent.SetCollisionEnabled` (`self.Door 1`) "QueryAndPhysics")
      (`PrimitiveComponent.SetCollisionEnabled` (`self.Door 2`) "QueryAndPhysics"))))

(event `/Game/BlueprintCommun/BPI_Interact.Interact`
  (params (PlayerRef :type "/Game/Assets/Blueprint/Player/BP_Player Object Reference"))
  (if (and (not (`self.Is open`)) (>= (`/Game/Assets/Blueprint/Player/BP_Player.Money` (`self.As BP Player`)) (`self.Buy cost`)))
    (`/Game/Assets/Blueprint/Player/BP_Player.SetMoney` (`self.As BP Player`) (- (`/Game/Assets/Blueprint/Player/BP_Player.Money` (`self.As BP Player`)) (`self.Buy cost`)))
    (for _array_element (`self.All Doors`)
      (set `/Game/MathisDENAMUR/BP_UnlockableDoor.Buy cost` (+ (`/Game/MathisDENAMUR/BP_UnlockableDoor.Buy cost` _array_element) 250) _array_element))
    (`GameplayStatics.PlaySound2D` "/Game/CHARONNAT/SoundDesign/Sounds/Player/Door/A_Door_Cue.A_Door_Cue" 1.0 1.0 0.0 null null)
    (if (`self.Lier ?`)
      (`self.open` (`self.Door linked`))
      (goto _label)
      (else
        (goto _label)))))

(event `/Game/BATET/Bp_buyitem/BPI_AffUI.AffUi`
  (params (PlayerRef :type "/Game/Assets/Blueprint/Player/BP_Player Object Reference"))
  (set `/Game/BATET/Widget/WBP_LockDoor.As BP Player` PlayerRef (`self.As WBP Lock Door`))
  (if (`self.Is open`)
    (`SceneComponent.SetVisibility` (`self.OpenDoor`) false false)
    (else
      (`SceneComponent.SetVisibility` (`self.LockDoor`) true false))))

(event `/Game/BATET/Bp_buyitem/BPI_AffUI.StopUi`
  (params (PlayerRef :type "/Game/Assets/Blueprint/Player/BP_Player Object Reference"))
  (set `/Game/BATET/Widget/WBP_LockDoor.As BP Player` PlayerRef (`self.As WBP Lock Door`))
  (`SceneComponent.SetVisibility` (`self.OpenDoor`) false false)
  (`SceneComponent.SetVisibility` (`self.LockDoor`) false false))

(fn `UserConstructionScript`
  (bind _door_2 (`self.Door 2`))
  (bind _door_1 (`self.Door 1`))
  (if (`self.Double porte`)
    (`StaticMeshComponent.SetStaticMesh` (`self.Encadrement`) "/Game/Hospital_Meshingun/Environment/Asset/Mesh/Props/Door/SM_Door_Frame_Cracked_04b.SM_Door_Frame_Cracked_04b")
    (`StaticMeshComponent.SetStaticMesh` _door_2 "/Game/Hospital_Meshingun/Environment/Asset/Mesh/Props/Door/SM_Door_Plate_02a.SM_Door_Plate_02a")
    (`SceneComponent.K2_SetRelativeLocation` _door_2 (0.0 11.0 0.0) false false)
    (`StaticMeshComponent.SetStaticMesh` _door_1 "/Game/Hospital_Meshingun/Environment/Asset/Mesh/Props/Door/SM_Door_Plate_02a.SM_Door_Plate_02a")
    (`SceneComponent.K2_SetRelativeLocation` _door_1 (0.0 -210.0 0.0) false false)))