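; BP_AllTheCodes is a scratch Blueprint holding placeholder scoring code for zombie kills.
; Its DeadZombie event adds points to Score from the actor's distance to RefPlayer, scaled by a per-weapon multiplier and a bone-hit multiplier.
; The visibility line trace is unwired placeholder shooting code, and the bone check is hardcoded true, so the bonus multiplier always applies.
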(event `DeadZombie`
  ;[1 1 1] SCORING CODE
  ;;[1 1 1] The code for shooting the boollet (placeholder)
  (bind _outhit (`KismetSystemLibrary.LineTraceSingle` (0.0 0.0 0.0) (0.0 0.0 0.0) "TraceTypeQuery1"))
  ;;[1 1 1] Score Calculations
  (if true
    (set `self.BoneMultiplier` 1.5)
    (else
      (set `self.BoneMultiplier` 1.0)))
  (set `self.Score` (+ (`self.Score`) (* (`self.GetDistanceTo` self (`self.RefPlayer`)) 100.0 (`|GetArrayItem` (`self.WeaponMultiplier`) (`self.weaponIndex`)) (`self.BoneMultiplier`)))))

(fn `UserConstructionScript`)