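; Vending machine that sells the player a Mastodonte, Stamina or Double Hit drink, with material and price set by machine type.
; An overlap sphere runs a looping timer that flags whether the player faces the machine, using a dot-product threshold that tightens with distance.
; Interact requires that flag and enough money, then deducts the price, spawns and starts a matching BP_Drink, and briefly blocks repeat purchases.
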(event `self.ReceiveBeginPlay`
  (bind _returnvalue (`KismetSystemLibrary.K2_SetTimer` null "IsPlayerLooking?" 0.1 true))
  (bind _output_get (set `self.PlayerLookTimer` _returnvalue))
  (`KismetSystemLibrary.K2_PauseTimerHandle` _output_get)
  (set `self.price` (select `/Game/BERNAGuillaume/VendingMachine/EnumVendingMachineType` (`self.VendingMachineType`) :`NewEnumerator0` 3000 :`NewEnumerator1` 3000 :`NewEnumerator2` 5000)))

(event `/Game/BlueprintCommun/BPI_Interact.Interact`
  (params (PlayerRef :type "/Game/Assets/Blueprint/Player/BP_Player Object Reference"))
  (bind _as_bp_player (`self.As BP Player`))
  (bind _returnvalue (`SceneComponent.K2_GetComponentToWorld` (`self.DrinkSpawnScene`)))
  (bind _returnvalue_2 (select `/Game/BERNAGuillaume/VendingMachine/EnumVendingMachineType` (`self.VendingMachineType`) :`NewEnumerator0` "/Game/BERNAGuillaume/Drinks/Models/MI_MastCan.MI_MastCan" :`NewEnumerator1` "/Game/BERNAGuillaume/Drinks/Models/MI_StamCan.MI_StamCan" :`NewEnumerator2` "/Game/BERNAGuillaume/Drinks/Models/Mi_DoHiCan.Mi_DoHiCan" :!type "MaterialInstance Object Reference"))
  (if (and (`self.IsLooking`) (>= (`/Game/Assets/Blueprint/Player/BP_Player.Money` (`self.As BP Player`)) (`self.price`)) (not (`self.StopBuying`)))
    (set `self.StopBuying` true)
    (`/Game/Assets/Blueprint/Player/BP_Player.SetMoney` _as_bp_player (- (`/Game/Assets/Blueprint/Player/BP_Player.Money` _as_bp_player) (`self.price`)))
    (`KismetSystemLibrary.K2_SetTimerDelegate` (delegate `DontBuyTwice!`) 3.0)
    (switch `/Game/BERNAGuillaume/VendingMachine/EnumVendingMachineType` (`self.VendingMachineType`)
      (:`NewEnumerator0`
        (bind _returnvalue_3 (`|SpawnActorFromClass` "/Game/BERNAGuillaume/Drinks/BP_Drink.BP_Drink_C" _returnvalue "Undefined" "MultiplyWithRoot" null null))
        (set `/Game/BERNAGuillaume/Drinks/BP_Drink.DrinkType` "NewEnumerator0" _returnvalue_3)
        (set `/Game/BERNAGuillaume/Drinks/BP_Drink.As BP Player` (`self.As BP Player`) _returnvalue_3)
        (bind _staticmeshcan (`/Game/BERNAGuillaume/Drinks/BP_Drink.StaticMeshCan` _returnvalue_3)
          (:`then`
            (`PrimitiveComponent.SetMaterial` _staticmeshcan 0 _returnvalue_2)
            (`/Game/BERNAGuillaume/Drinks/BP_Drink.DrinkStart` _returnvalue_3))
          (:`else`)))
      (:`NewEnumerator1`
        (bind _returnvalue_4 (`|SpawnActorFromClass` "/Game/BERNAGuillaume/Drinks/BP_Drink.BP_Drink_C" _returnvalue "Undefined" "MultiplyWithRoot" null null))
        (set `/Game/BERNAGuillaume/Drinks/BP_Drink.DrinkType` "NewEnumerator1" _returnvalue_4)
        (set `/Game/BERNAGuillaume/Drinks/BP_Drink.As BP Player` (`self.As BP Player`) _returnvalue_4)
        (bind _staticmeshcan_2 (`/Game/BERNAGuillaume/Drinks/BP_Drink.StaticMeshCan` _returnvalue_4)
          (:`then`
            (`PrimitiveComponent.SetMaterial` _staticmeshcan_2 0 _returnvalue_2)
            (`/Game/BERNAGuillaume/Drinks/BP_Drink.DrinkStart` _returnvalue_4))
          (:`else`)))
      (:`NewEnumerator2`
        (bind _returnvalue_5 (`|SpawnActorFromClass` "/Game/BERNAGuillaume/Drinks/BP_Drink.BP_Drink_C" _returnvalue "Undefined" "MultiplyWithRoot" null null))
        (set `/Game/BERNAGuillaume/Drinks/BP_Drink.DrinkType` "NewEnumerator2" _returnvalue_5)
        (set `/Game/BERNAGuillaume/Drinks/BP_Drink.As BP Player` (`self.As BP Player`) _returnvalue_5)
        (bind _staticmeshcan_3 (`/Game/BERNAGuillaume/Drinks/BP_Drink.StaticMeshCan` _returnvalue_5)
          (:`then`
            (`PrimitiveComponent.SetMaterial` _staticmeshcan_3 0 _returnvalue_2)
            (`/Game/BERNAGuillaume/Drinks/BP_Drink.DrinkStart` _returnvalue_5))
          (:`else`))))))

(event `DontBuyTwice!`
  (set `self.StopBuying` false))

(event `self.Sphere.OnComponentBeginOverlap`
  (params (OverlappedComponent :type "PrimitiveComponent Object Reference") (OtherActor :type "Actor Object Reference") (OtherComp :type "PrimitiveComponent Object Reference") (OtherBodyIndex :type Integer) (bFromSweep :type Boolean) (SweepResult :type "HitResult Structure (by ref)"))
  (if (not (`self.PlayerSetup?`))
    (bind _asbp_player (cast `/Game/Assets/Blueprint/Player/BP_Player` OtherActor))
    (set `self.As BP Player` _asbp_player)
    (set `self.PlayerSetup?` true)
    (`KismetSystemLibrary.K2_UnPauseTimerHandle` (`self.PlayerLookTimer`))
    (else
      (cast `/Game/Assets/Blueprint/Player/BP_Player` OtherActor)
      (`KismetSystemLibrary.K2_UnPauseTimerHandle` (`self.PlayerLookTimer`)))))

(event `self.Sphere.OnComponentEndOverlap`
  (params (OverlappedComponent :type "PrimitiveComponent Object Reference") (OtherActor :type "Actor Object Reference") (OtherComp :type "PrimitiveComponent Object Reference") (OtherBodyIndex :type Integer))
  (`KismetSystemLibrary.K2_PauseTimerHandle` (`self.PlayerLookTimer`)))

(fn `IsPlayerLooking?`
  (bind _vendingmachinemesh (`self.VendingMachineMesh`))
  (bind _camera (`/Game/Assets/Blueprint/Player/BP_Player.Camera` (`self.As BP Player`)))
  (if (< (`KismetMathLibrary.Dot_VectorVector` (`SceneComponent.GetForwardVector` _camera) (`SceneComponent.GetRightVector` _vendingmachinemesh)) (`KismetMathLibrary.Lerp` -0.5 -1.0 (/ (`KismetMathLibrary.Vector_Distance` (`SceneComponent.K2_GetComponentLocation` _camera) (`SceneComponent.K2_GetComponentLocation` _vendingmachinemesh)) 360.0)))
    (`/Engine/EditorBlueprintResources/StandardMacros.DoOnce` false :!label _label
      (:`Completed`
        (set `self.IsLooking` true)
        (goto _label_2 :!via `Reset`)))
    (else
      (`/Engine/EditorBlueprintResources/StandardMacros.DoOnce` false :!label _label_2
        (:`Completed`
          (set `self.IsLooking` false)
          (goto _label :!via `Reset`))))))

(fn `UserConstructionScript`
  (bind _vendingmachinemesh (`self.VendingMachineMesh`))
  (bind (_returnvalue_location _returnvalue_rotation) (`KismetMathLibrary.BreakTransform` (`SceneComponent.K2_GetComponentToWorld` _vendingmachinemesh)))
  (`StaticMeshComponent.SetStaticMesh` (`self.VendingMachineMesh`) (select `/Game/BERNAGuillaume/VendingMachine/EnumVendingMachineType` (`self.VendingMachineType`) :`NewEnumerator0` "/Game/BERNAGuillaume/VendingMachine/Models/Model/SM_VendingMachine1.SM_VendingMachine1" :`NewEnumerator1` "/Game/BERNAGuillaume/VendingMachine/Models/Model/SM_VendingMachine1.SM_VendingMachine1" :`NewEnumerator2` "/Game/BERNAGuillaume/VendingMachine/Models/Model/SM_VendingMachine1.SM_VendingMachine1" :!type "StaticMesh Object Reference"))
  (`PrimitiveComponent.SetMaterial` _vendingmachinemesh 0 (select `/Game/BERNAGuillaume/VendingMachine/EnumVendingMachineType` (`self.VendingMachineType`) :`NewEnumerator0` "/Game/BERNAGuillaume/VendingMachine/Models/MI_VendingMachine1.MI_VendingMachine1" :`NewEnumerator1` "/Game/BERNAGuillaume/VendingMachine/Models/MI_VendingMachine2.MI_VendingMachine2" :`NewEnumerator2` "/Game/BERNAGuillaume/VendingMachine/Models/MI_VendingMachine3.MI_VendingMachine3" :!type "MaterialInstance Object Reference"))
  (`SceneComponent.K2_SetWorldTransform` _vendingmachinemesh (`KismetMathLibrary.MakeTransform` _returnvalue_location _returnvalue_rotation (7.0 7.0 7.0)) false false))