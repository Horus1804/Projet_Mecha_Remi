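; BP_Drink is a drink can actor in three types (Mastodonte, Stamina, Double Hit), with the can material picked by type in the construction script.
; DrinkStart turns off can physics, snaps the can to its grab point and attaches it to a hand socket on the player's Hands mesh.
; It plays a drinking montage, calls the player's matching effect as playback starts, and destroys itself when the montage completes or is interrupted.
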(event `DrinkStart`
  (`self.ResetDrink`)
  (`self.SetDrinkToHand`)
  (`|PlayMontage` (`/Game/Assets/Blueprint/Player/BP_Player.Hands` (`self.As BP Player`)) "/Game/BERNAGuillaume/Animation/AS_DrinkingCanReal_Montage.AS_DrinkingCanReal_Montage"
    (:`then`
      (switch `/Game/BERNAGuillaume/VendingMachine/EnumVendingMachineType` (`self.DrinkType`)
        (:`NewEnumerator0`
          (`/Game/Assets/Blueprint/Player/BP_Player.DrinksMasto` (`self.As BP Player`)))
        (:`NewEnumerator1`
          (`/Game/Assets/Blueprint/Player/BP_Player.DrinksStamina` (`self.As BP Player`)))
        (:`NewEnumerator2`
          (`/Game/Assets/Blueprint/Player/BP_Player.DrinksDoubleHit` (`self.As BP Player`)))))
    (:`OnCompleted`
      (`self.K2_DestroyActor` :!label _label))
    (:`OnInterrupted`
      (goto _label))))

(event `ResetDrink`
  (`PrimitiveComponent.SetSimulatePhysics` (`self.StaticMeshCan`) false)
  (`SceneComponent.K2_AttachToComponent` (`self.StaticMeshCan`) (`self.GrabPoint`) "None" "SnapToTarget" "SnapToTarget" "KeepRelative" true))

(event `SetDrinkToHand`
  (bind _as_bp_player (`self.As BP Player`)
    (:`then`
      (bind _hands (`/Game/Assets/Blueprint/Player/BP_Player.Hands` _as_bp_player))
      (`self.K2_AttachToComponent` _hands (`SkinnedMeshComponent.GetSocketBoneName` _hands "HandWeapon_IK") "SnapToTarget" "SnapToTarget" "KeepRelative"))
    (:`else`)))

(fn `UserConstructionScript`
  (`PrimitiveComponent.SetMaterial` (`self.StaticMeshCan`) 0 (select `/Game/BERNAGuillaume/VendingMachine/EnumVendingMachineType` (`self.DrinkType`) :`NewEnumerator0` "/Game/BERNAGuillaume/Drinks/Models/MI_MastCan.MI_MastCan" :`NewEnumerator1` "/Game/BERNAGuillaume/Drinks/Models/MI_StamCan.MI_StamCan" :`NewEnumerator2` "/Game/BERNAGuillaume/Drinks/Models/Mi_DoHiCan.Mi_DoHiCan" :!type "MaterialInstance Object Reference")))