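; AK74 child weapon Blueprint that sets its own ammo, weapon type and fire rate on BeginPlay.
; Fire plays sound, muzzle flash, shell ejection and recoil, then line-traces from the barrel socket and sends damage through BPI_Shoot, with an InstaKill override.
; The flash light is a briefly lived spawned PointLight, replacing an unused component-based version.
; Split and ReSplit play a sequence forward and backward; Reload refills ammo.
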(event `self.ReceiveBeginPlay`
  (`parent.ReceiveBeginPlay`)
  (set `self.actualAmmo` 30)
  (`|VariableSetRef` (`self.WeaponType`) "NewEnumerator2")
  (set `self.fireRate` 0.09))

(event `self.Split`
  (`ActorSequenceComponent.PlaySequence` (`self.AS_Split`)))

(event `self.ReSplit`
  (`MovieSceneSequencePlayer.PlayReverse` (`ActorSequenceComponent.SequencePlayer` (`self.AS_Split`))))

(event `self.Fire`
  (bind _ak74_handle_low (`self.AK74_handle_low`))
  (bind _returnvalue (`SceneComponent.GetSocketLocation` _ak74_handle_low "BarrelEndSocket"))
  (if (!= (`self.actualAmmo`) 0)
    (`self.FireAnim`)
    (`self.CreateFlashMuzzle`)
    (`self.PlayRecoil`)
    (bind _outhit (`KismetSystemLibrary.LineTraceSingleForObjects` _returnvalue (+ _returnvalue (* (`KismetMathLibrary.GetForwardVector` (`SceneComponent.GetSocketRotation` _ak74_handle_low "BarrelEndSocket")) 1600.0)) (`|MakeArray` "ObjectTypeQuery3" "ObjectTypeQuery2" "ObjectTypeQuery4" :!type "EObjectTypeQuery Enum") false (`|MakeArray` (`GameplayStatics.GetPlayerPawn` 0) :!type "Actor Object Reference")))
    (`/Engine/EditorBlueprintResources/StandardMacros.DecrementInt` (`self.actualAmmo`)
      (:`  `
        (bind (_bblockinghit _binitialoverlap _time _distance _location _impactpoint _normal _impactnormal _physmat _hitactor) (`GameplayStatics.BreakHitResult` _outhit))
        (if (`KismetSystemLibrary.DoesImplementInterface` _hitactor "/Game/Weapon/BPI_Shoot.BPI_Shoot_C")
          (message `/Game/Weapon/BPI_Shoot.ShootHit` _hitactor _physmat _impactpoint self (select `bool` (`self.InstaKill`) :`false` (`self.damage`) :`true` 99999.0)))))))

(event `self.Reload`
  (set `self.actualAmmo` (`self.maxAmmo`)))

(event `FireAnim`
  (bind _bulleteject (`self.BulletEject`))
  (`GameplayStatics.PlaySoundAtLocation` "/Game/Weapon/SoundEffect/AK74/Cue_ak74FireSound.Cue_ak74FireSound" (`SceneComponent.GetSocketLocation` (`self.AK74_handle_low`) "BarrelEndSocket") (struct) 1.0 1.0 0.0 null null null null)
  (`ActorComponent.Activate` (`self.MuzzleFlashes`) true)
  (`NiagaraFunctionLibrary.SpawnSystemAtLocation` "/Game/Assets/Niagara/Gun_VFX/Niagara_FX/Bullet_ejection/NS_AR_Ejection_Effect.NS_AR_Ejection_Effect" (`SceneComponent.K2_GetComponentLocation` _bulleteject) (`KismetMathLibrary.MakeRotator` (.roll (`SceneComponent.K2_GetComponentRotation` _bulleteject)) (.pitch (`SceneComponent.K2_GetComponentRotation` _bulleteject)) (+ (.yaw (`SceneComponent.K2_GetComponentRotation` _bulleteject)) 45.0))))

(event `CreateFlashMuzzle`
  (bind _returnvalue (`|SpawnActorFromClass` "/Script/Engine.PointLight" (`KismetMathLibrary.MakeTransform` (0.0 0.0 0.0)) "AlwaysSpawn" "MultiplyWithRoot" null null))
  (`self.K2_AttachToComponent` _returnvalue (`self.AK74_handle_low`) "BarrelEndSocket" "SnapToTarget" "SnapToTarget" "KeepRelative" true)
  (`self.SetLifeSpan` _returnvalue 0.05))

(fn `UserConstructionScript`
  (`parent.UserConstructionScript`))