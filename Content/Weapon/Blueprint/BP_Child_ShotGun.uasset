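; Shotgun child weapon Blueprint that fires a hitscan spread of pellets and sets its own weapon type, fire rate and starting ammo.
; Each shot plays shell-ejection Niagara and sound, then runs looped line traces from the barrel socket with random spread, ignoring the player pawn.
; Hit actors implementing BPI_Shoot receive damage, boosted massively under InstaKill.
; A shot costs one round, and Reload instantly refills to MaxAmmo.
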(event `self.ReceiveBeginPlay`
  (`parent.ReceiveBeginPlay`)
  (set `self.actualAmmo` 5)
  (`|VariableSetRef` (`self.WeaponType`) "NewEnumerator3")
  (set `self.fireRate` 0.8))

(event `self.Fire`
  (bind _body (`self.Body`))
  (bind _spreed (`self.Spreed`))
  (bind _spreed_2 (`self.Spreed`))
  (bind _spreed_3 (`self.Spreed`))
  (bind _returnvalue (`SceneComponent.GetSocketLocation` _body "BarrelEndSocket"))
  (if (!= (`self.actualAmmo`) 0)
    (`self.FireAnim`)
    (for _ (range 11)
      (bind _outhit (`KismetSystemLibrary.LineTraceSingleForObjects` _returnvalue (+ _returnvalue (* (`KismetMathLibrary.GetForwardVector` (`SceneComponent.GetSocketRotation` _body "BarrelEndSocket")) 1600.0) (`KismetMathLibrary.MakeVector` (`KismetMathLibrary.RandomFloatInRange` (* _spreed_2 -1.0) _spreed_2) (`KismetMathLibrary.RandomFloatInRange` (* _spreed_3 -1.0) _spreed_3) (`KismetMathLibrary.RandomFloatInRange` (* _spreed -1.0) _spreed))) (`|MakeArray` "ObjectTypeQuery3" "ObjectTypeQuery4" "ObjectTypeQuery2" :!type "EObjectTypeQuery Enum") false (`|MakeArray` (`GameplayStatics.GetPlayerPawn` 0) :!type "Actor Object Reference")))
      (bind (_bblockinghit _binitialoverlap _time _distance _location _impactpoint _normal _impactnormal _physmat _hitactor) (`GameplayStatics.BreakHitResult` _outhit))
      (if (`KismetSystemLibrary.DoesImplementInterface` _hitactor "/Game/Weapon/BPI_Shoot.BPI_Shoot_C")
        (message `/Game/Weapon/BPI_Shoot.ShootHit` _hitactor _physmat _impactpoint self (select `bool` (`self.InstaKill`) :`false` (`self.damage`) :`true` 9999999.0))))
    (`/Engine/EditorBlueprintResources/StandardMacros.DecrementInt` (`self.actualAmmo`))))

(event `self.Reload`
  (set `self.actualAmmo` (`self.maxAmmo`)))

(event `FireAnim`
  (bind _shelleject (`self.ShellEject`))
  (`NiagaraFunctionLibrary.SpawnSystemAtLocation` "/Game/Assets/Niagara/Gun_VFX/Niagara_FX/Bullet_ejection/NS_Shotgun_Ejection_Effect.NS_Shotgun_Ejection_Effect" (`SceneComponent.K2_GetComponentLocation` _shelleject) (`KismetMathLibrary.MakeRotator` (.roll (`SceneComponent.K2_GetComponentRotation` _shelleject)) (.pitch (`SceneComponent.K2_GetComponentRotation` _shelleject)) (+ (.yaw (`SceneComponent.K2_GetComponentRotation` _shelleject)) 45.0)))
  (`GameplayStatics.SpawnSoundAttached` "/Game/Weapon/SoundEffect/Remington870/Cue_ShotGunFireReload.Cue_ShotGunFireReload" (`self.Body`) "BarrelEndSocket" (0.0 0.0 0.0) (struct) "SnapToTarget" false 1.0 1.0 0.0 null null))

(fn `UserConstructionScript`
  (`parent.UserConstructionScript`))