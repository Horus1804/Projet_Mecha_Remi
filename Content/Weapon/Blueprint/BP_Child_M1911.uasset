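; M1911 pistol, a child weapon Blueprint that handles firing, reloading and ammo count, with a debug ammo print each tick.
; Fire plays slide timeline, recoil, audio, Niagara effects and a short-lived muzzle light, then traces from the barrel along camera forward.
; Hit actors implementing BPI_Shoot receive damage, or an InstaKill value, plus the physical material as hit zone.
; Separate events eject the clip and play the ASSplit sequence forward or reverse.
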(event `self.ReceiveBeginPlay`
  (`parent.ReceiveBeginPlay`)
  (set `self.actualAmmo` 6)
  (`|VariableSetRef` (`self.WeaponType`) "NewEnumerator1")
  (set `self.fireRate` 0.0))

(event `self.ReceiveTick`
  (params (DeltaSeconds :type "Float (single-precision)"))
  (`parent.ReceiveTick` DeltaSeconds)
  (`KismetSystemLibrary.PrintString` (`KismetStringLibrary.Concat_StrStr` "Actual ammo 1911" " -- " (`KismetStringLibrary.Conv_IntToString` (`self.actualAmmo`))) true true (struct :`G` 1.0 :`B` 0.130324 :`A` 1.0) 0.0))

(event `self.Split`
  (`ActorSequenceComponent.PlaySequence` (`self.AS_Split`)))

(event `/Game/Weapon/BPI_Shoot.ShootHit`
  (params (HitZone :type "PhysicalMaterial Object Reference") (HitLocation :type "Vector Structure") (Causer :type "Actor Object Reference") (BaseDamage :type "Float (double-precision)"))
  (set `self.Hit Location` HitLocation))

(event `self.ReSplit`
  (`MovieSceneSequencePlayer.PlayReverse` (`ActorSequenceComponent.SequencePlayer` (`self.AS_Split`))))

(event `self.Fire`
  (bind _returnvalue (`SceneComponent.GetSocketLocation` (`self.M1911Fix_barrel`) "BarrelEndSocket"))
  (`self.FireAnim`)
  (`self.CreateFlashMuzzle`)
  (`self.PlayRecoil`)
  (bind _returnvalue_2 (`NiagaraFunctionLibrary.SpawnSystemAtLocation` "/Game/Assets/Niagara/Gun_VFX/Niagara_FX/Bullet_ejection/NS_Pistol_Ejection_Effect.NS_Pistol_Ejection_Effect" (`SceneComponent.K2_GetComponentLocation` (`self.Ejection_Bullet`)) (`SceneComponent.K2_GetComponentRotation` (`self.Arrow`))))
  (`PrimitiveComponent.SetCastShadow` _returnvalue_2 true)
  (`AudioComponent.Play` (`self.FireAudio`) 0.0)
  (`ActorComponent.Activate` (`self.NS_Pistol_Muzzle_flashes_02`) true)
  (bind _outhit (`KismetSystemLibrary.LineTraceSingleForObjects` _returnvalue (+ _returnvalue (* (`self.GetActorForwardVector` (`GameplayStatics.GetPlayerCameraManager` 0)) 1600.0)) (`|MakeArray` "ObjectTypeQuery3" "ObjectTypeQuery4" "ObjectTypeQuery2" :!type "EObjectTypeQuery Enum") false (`|MakeArray` (`GameplayStatics.GetPlayerPawn` 0) :!type "Actor Object Reference")))
  (`/Engine/EditorBlueprintResources/StandardMacros.DecrementInt` (`self.actualAmmo`)
    (:`  `
      (bind (_bblockinghit _binitialoverlap _time _distance _location _impactpoint _normal _impactnormal _physmat _hitactor) (`GameplayStatics.BreakHitResult` _outhit))
      (if (`KismetSystemLibrary.DoesImplementInterface` _hitactor "/Game/Weapon/BPI_Shoot.BPI_Shoot_C")
        (message `/Game/Weapon/BPI_Shoot.ShootHit` _hitactor _physmat _impactpoint self (select `bool` (`self.InstaKill`) :`false` (`self.damage`) :`true` 9999999.0))))))

(event `self.Reload`
  (set `self.actualAmmo` (`self.maxAmmo`)))

(event `self.EjectClipToReload`
  (bind _returnvalue (`NiagaraFunctionLibrary.SpawnSystemAtLocation` "/Game/Assets/Niagara/Gun_VFX/Niagara_FX/Reload_Fx/NS_1911ClipEject.NS_1911ClipEject" (`SceneComponent.K2_GetComponentLocation` (`self.ClipEject`))))
  (`FXSystemComponent.SetVectorParameter` _returnvalue "VelocityEjectClip" (* (`KismetMathLibrary.GetForwardVector` (`SceneComponent.K2_GetComponentRotation` (`self.ClipEject`))) 100.0)))

(event `FireAnim`
  (bind (_direction _slidefire) (`Timeline|FireAnimTimeLine` :!via `PlayFromStart` :!label _label)
    (:`Update`
      (`SceneComponent.K2_SetRelativeLocation` (`self.M1911Fix_slide`) _slidefire false false))
    (:`Finished`
      (`self.FireAnimEnd`))))

(event `FireAnimEnd`
  (goto _label :!via `Reverse`))

(event `CreateFlashMuzzle`
  (bind _returnvalue (`|SpawnActorFromClass` "/Script/Engine.PointLight" (`KismetMathLibrary.MakeTransform` (0.0 0.0 0.0)) "AlwaysSpawn" "MultiplyWithRoot" null null))
  (`self.K2_AttachToComponent` _returnvalue (`self.M1911Fix_barrel`) "BarrelEndSocket" "SnapToTarget" "SnapToTarget" "KeepRelative" true)
  (`self.SetLifeSpan` _returnvalue 0.05))

(fn `UserConstructionScript`
  (`parent.UserConstructionScript`))