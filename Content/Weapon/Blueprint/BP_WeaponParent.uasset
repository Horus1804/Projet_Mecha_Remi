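; Base weapon Blueprint for a player pickup with ammo, procedural recoil and Pack-a-Punch upgrades, leaving fire and reload events empty.
; Interact destroys the equipped weapon when slot 1 is filled, then adds and equips this one unless it is on Pack-a-Punch, disabling its interaction collision.
; Upgrade spends player money to raise a global level, reading damage, aim, max ammo and load-failure stats from a data asset.
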(event `SetPivot`
  ;[0.2717 0.3542 0] Set Good Location & Rotation
  (`self.Player`
    (:`then`
      (`SceneComponent.K2_SetRelativeLocationAndRotation` (`self.Root`) (`self.LocationHandIK`) (`self.RotationHandIK`) false true))
    (:`else`)))

(event `self.ReceiveBeginPlay`
  (bind _maxammo (`self.maxAmmo`))
  (set `self.StockAmmo` _maxammo)
  (set `self.actualAmmo` _maxammo))

(event `EjectClipToReload`)

(event `Fire`)

(event `Reload`)

(event `ReSplit`)

(event `Split`)

(event `InitialRecoil`
  ;[1 0.4863 0.2222] Recoil Procedural
  (bind _player (`self.Player`)
    (:`then`
      (`RecoilAnimationComponent.Init` (`/Game/Assets/Blueprint/Player/BP_Player.RecoilAnimation` _player) (`.Recoil_3_6F3D9E064A534B31FC8429B4122AA8F6` (break `/Game/Assets/Blueprint/WeaponsRecoil/ST_ProceduralRecoil` (`self.DataRecoil`))) 600.0 0))
    (:`else`)))

(event `/Game/BlueprintCommun/BPI_Interact.Interact`
  (params (PlayerRef :type "/Game/Assets/Blueprint/Player/BP_Player Object Reference"))
  (bind _weaponsslot (`/Game/Assets/Blueprint/Player/BP_Player.WeaponsSlot` PlayerRef))
  (bind _output (`|GetArrayItem` _weaponsslot (`KismetMathLibrary.Conv_BoolToInt` (`/Game/Assets/Blueprint/Player/BP_Player.WeaponsEquiped` PlayerRef))))
  (`/Engine/EditorBlueprintResources/StandardMacros.IsValid` (`|GetArrayItem` _weaponsslot 1)
    (:`Is Valid`
      (set `self.WeaponSlot` _output)
      (`KismetArrayLibrary.Array_Remove` _weaponsslot (`KismetArrayLibrary.Array_Find` _weaponsslot _output))
      (`self.K2_DestroyActor` (`self.WeaponSlot`)))
    (:`Is Not Valid`
      _))
  (`self.AddItem` PlayerRef))

(event `PlayRecoil`
  ;[1 0.4863 0.2222] Recoil Procedural
  (bind _player (`self.Player`)
    (:`then`
      (`RecoilAnimationComponent.Play` (`/Game/Assets/Blueprint/Player/BP_Player.RecoilAnimation` _player)))
    (:`else`)))

(event `AddItem`
  (params (Player :type "/Game/Assets/Blueprint/Player/BP_Player Object Reference"))
  ;[0.2754 0.2314 1] Interact With Weapons
  (if (not (`self.IsOnPackAPunch`))
    (bind _output_get (set `self.Player` Player))
    (`KismetArrayLibrary.Array_AddUnique` (`/Game/Assets/Blueprint/Player/BP_Player.WeaponsSlot` Player) self)
    (`/Engine/EditorBlueprintResources/StandardMacros.IsValid` _output_get
      (:`Is Valid`
        (`/Game/Assets/Blueprint/Player/BP_Player.Equipe Weapon` _output_get self)
        (`self.DisableInteractionStaticMeshComponent`)
        (set `self.IsTaken` true)))))

(event `StopRecoil`
  ;[1 0.4863 0.2222] Recoil Procedural
  (bind _player (`self.Player`)
    (:`then`
      (`RecoilAnimationComponent.Stop` (`/Game/Assets/Blueprint/Player/BP_Player.RecoilAnimation` _player)))
    (:`else`)))

(event `Upgrade`
  (params (UpgradeType :type "/Game/ALBERLATOUR/EUpgradeType Enum" :default "NewEnumerator0"))
  (bind _money (`/Game/Assets/Blueprint/Player/BP_Player.Money` (`self.Player`)))
  (bind (_value _returnvalue) (`BlueprintMapLibrary.Map_Find` (`/Game/Weapon/Blueprint/Data/PDA_Weapon.ratioLoadFailed` (`self.DA_Stats`)) (`self.LevelGlobalWeapon`)))
  (bind (_value_2 _returnvalue_2) (`BlueprintMapLibrary.Map_Find` (`/Game/Weapon/Blueprint/Data/PDA_Weapon.Aim` (`self.DA_Stats`)) (`self.LevelGlobalWeapon`)))
  (bind _value_3 (`BlueprintMapLibrary.Map_Find` (`/Game/Weapon/Blueprint/Data/PDA_Weapon.Cost` (`self.DA_Stats`)) (`self.LevelGlobalWeapon`)))
  (bind (_value_4 _returnvalue_3) (`BlueprintMapLibrary.Map_Find` (`/Game/Weapon/Blueprint/Data/PDA_Weapon.Damage` (`self.DA_Stats`)) (`self.LevelGlobalWeapon`)))
  (bind (_value_5 _returnvalue_4) (`BlueprintMapLibrary.Map_Find` (`/Game/Weapon/Blueprint/Data/PDA_Weapon.MaxAmmo` (`self.DA_Stats`)) (`self.LevelGlobalWeapon`)))
  ;[0.6466 0.333 1] Upgrade Weapons
  (switch `/Game/ALBERLATOUR/EUpgradeType` UpgradeType
    (:`NewEnumerator4`
      (if (>= _money _value_3)
        (`/Game/Assets/Blueprint/Player/BP_Player.SetMoney` (`self.Player`) (- _money _value_3))
        (`/Engine/EditorBlueprintResources/StandardMacros.IncrementInt` (`self.LevelGlobalWeapon`)
          (:`  `
            (`|ExecutionSequence`
              (:`then_0`
                (if _returnvalue_3
                  (bind _output_get (set `self.damage` _value_4))
                  (`KismetSystemLibrary.PrintString` (`KismetStringLibrary.Conv_DoubleToString` _output_get))))
              (:`then_1`
                (if _returnvalue_2
                  (bind _output_get_2 (set `self.aim` _value_2))
                  (`KismetSystemLibrary.PrintString` (`KismetStringLibrary.Conv_DoubleToString` _output_get_2))))
              (:`then_2`
                (if _returnvalue_4
                  (bind _output_get_3 (set `self.maxAmmo` _value_5))
                  (`KismetSystemLibrary.PrintString` (`KismetStringLibrary.Conv_IntToString` _output_get_3))))
              (:`then_3`
                (if _returnvalue
                  (bind _output_get_4 (set `self.ratioLoadFailed` _value))
                  (`KismetSystemLibrary.PrintString` (`KismetStringLibrary.Conv_DoubleToString` _output_get_4)))))))))))

(fn `DisableInteractionStaticMeshComponent`
  ;[1 0.191 0.3513] Disable Component Collision
  (if (`KismetArrayLibrary.Array_IsNotEmpty` (`self.ComponentMesh`))
    (for _array_element (`self.ComponentMesh`)
      (`PrimitiveComponent.SetCollisionResponseToChannel` _array_element "ECC_GameTraceChannel1" "ECR_Ignore")))
  ;[1 0.9908 0] Disable Main Collision Target
  (`PrimitiveComponent.SetCollisionResponseToChannel` (`self.Box`) "ECC_GameTraceChannel1" "ECR_Ignore"))

(fn `GetOnPackAPunch`
  (returns (IsOnPackAPunch :type Boolean))
  (return (`self.IsOnPackAPunch`)))

(fn `SetOnPackAPunch`
  (params (IsOnPackAPunch :type Boolean))
  (set `self.IsOnPackAPunch` IsOnPackAPunch))

(fn `UserConstructionScript`
  (bind _returnvalue (`self.K2_GetComponentsByClass` "/Script/Engine.StaticMeshComponent"))
  ;[1 0.231 0.3408] Get All Components Static Mesh
  (if (`KismetArrayLibrary.Array_IsNotEmpty` _returnvalue)
    (set `self.ComponentMesh` _returnvalue)))