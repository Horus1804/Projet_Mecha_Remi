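; HK416 child weapon that sets ammo, weapon type and fire rate on BeginPlay and refills ammo on reload.
; Fire traces from the barrel socket and sends hit zone and damage, or an InstaKill value, through BPI_Shoot.
; Sound, muzzle flash and a short-lived spawned light follow the suppressor or barrel socket, alongside Niagara shell ejection.
; An Actor Sequence plays split and reverse; Tick draws leftover-style location debug output.
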(event `self.ReceiveBeginPlay`
  (`parent.ReceiveBeginPlay`)
  (set `self.actualAmmo` 30)
  (`|VariableSetRef` (`self.WeaponType`) "NewEnumerator6")
  (set `self.fireRate` 0.07))

(event `self.ReceiveTick`
  (params (DeltaSeconds :type "Float (single-precision)"))
  (bind (_returnvalue_location _returnvalue_rotation) (`KismetMathLibrary.BreakTransform` (`SceneComponent.K2_GetComponentToWorld` (`self.HK416Fix_HK416_Body`))))
  (`parent.ReceiveTick` DeltaSeconds)
  (`KismetSystemLibrary.PrintString` (`KismetStringLibrary.Conv_VectorToString` (`self.K2_GetActorLocation`)) true true (struct :`R` 1.0 :`G` 0.891671 :`B` 0.59482 :`A` 1.0) 0.0)
  (`KismetSystemLibrary.DrawDebugCoordinateSystem` _returnvalue_location _returnvalue_rotation 10.0 0.0 1.0))

(event `self.Split`
  (`ActorSequenceComponent.PlaySequence` (`self.ActorSequenceSplit`)))

(event `self.ReSplit`
  (`MovieSceneSequencePlayer.PlayReverse` (`ActorSequenceComponent.SequencePlayer` (`self.ActorSequenceSplit`))))

(event `self.Fire`
  (bind _hk416fix_barrel (`self.HK416Fix_Barrel`))
  (bind _returnvalue (`SceneComponent.GetSocketLocation` _hk416fix_barrel "BarrelEndSocket"))
  (if (!= (`self.actualAmmo`) 0)
    (`self.FireAnim`)
    (`self.CreateFlashMuzzle`)
    (bind _outhit (`KismetSystemLibrary.LineTraceSingleForObjects` _returnvalue (+ _returnvalue (* (`KismetMathLibrary.GetForwardVector` (`SceneComponent.GetSocketRotation` _hk416fix_barrel "BarrelEndSocket")) 1600.0)) (`|MakeArray` "ObjectTypeQuery3" "ObjectTypeQuery4" "ObjectTypeQuery2" :!type "EObjectTypeQuery Enum") false (`|MakeArray` (`GameplayStatics.GetPlayerPawn` 0) :!type "Actor Object Reference")))
    (`/Engine/EditorBlueprintResources/StandardMacros.DecrementInt` (`self.actualAmmo`)
      (:`  `
        (bind (_bblockinghit _binitialoverlap _time _distance _location _impactpoint _normal _impactnormal _physmat _hitactor) (`GameplayStatics.BreakHitResult` _outhit))
        (if (`KismetSystemLibrary.DoesImplementInterface` _hitactor "/Game/Weapon/BPI_Shoot.BPI_Shoot_C")
          (message `/Game/Weapon/BPI_Shoot.ShootHit` _hitactor _physmat _impactpoint self (select `bool` (`self.InstaKill`) :`false` (`self.damage`) :`true` 99999.0)))))))

(event `self.Reload`
  (set `self.actualAmmo` (`self.maxAmmo`)))

(event `FireAnim`
  (bind _bulleteject (`self.BulletEject`))
  (if (`self.SuppressorGet`)
    (`GameplayStatics.PlaySoundAtLocation` "/Game/Weapon/SoundEffect/HK416/Cue_HK416FireSoundRandom.Cue_HK416FireSoundRandom" (`SceneComponent.GetSocketLocation` (`self.HK416Fix_SuppressorClothWrap`) "SuppressorEndSocket") (struct) 1.0 1.0 0.0 null null null null)
    (`SceneComponent.K2_AttachToComponent` (`self.Muzzle_Flashes`) (`self.HK416Fix_SuppressorClothWrap`) "SuppressorEndSocket" "SnapToTarget" "SnapToTarget" "KeepRelative" true)
    (else
      (`GameplayStatics.PlaySoundAtLocation` "/Game/Weapon/SoundEffect/HK416/Cue_HK416FireSoundRandom.Cue_HK416FireSoundRandom" (`SceneComponent.GetSocketLocation` (`self.HK416Fix_Barrel`) "BarrelEndSocket") (struct) 1.0 1.0 0.0 null null null null)
      (`SceneComponent.K2_AttachToComponent` (`self.Muzzle_Flashes`) (`self.HK416Fix_Barrel`) "BarrelEndSocket" "SnapToTarget" "SnapToTarget" "KeepRelative" true)))
  (`ActorComponent.Activate` (`self.Muzzle_Flashes`) true)
  (`NiagaraFunctionLibrary.SpawnSystemAtLocation` "/Game/Assets/Niagara/Gun_VFX/Niagara_FX/Bullet_ejection/NS_AR_Ejection_Effect.NS_AR_Ejection_Effect" (`SceneComponent.K2_GetComponentLocation` _bulleteject) (`KismetMathLibrary.MakeRotator` (.roll (`SceneComponent.K2_GetComponentRotation` _bulleteject)) (.pitch (`SceneComponent.K2_GetComponentRotation` _bulleteject)) (+ (.yaw (`SceneComponent.K2_GetComponentRotation` _bulleteject)) 45.0))))

(event `CreateFlashMuzzle`
  (bind _returnvalue (`|SpawnActorFromClass` "/Script/Engine.PointLight" (`KismetMathLibrary.MakeTransform` (0.0 0.0 0.0)) "AlwaysSpawn" "MultiplyWithRoot" null null))
  (if (`self.SuppressorGet`)
    (`self.K2_AttachToComponent` _returnvalue (`self.HK416Fix_SuppressorClothWrap`) "SuppressorEndSocket" "SnapToTarget" "SnapToTarget" "KeepRelative" true)
    (else
      (`self.K2_AttachToComponent` _returnvalue (`self.HK416Fix_Barrel`) "BarrelEndSocket" "SnapToTarget" "SnapToTarget" "KeepRelative" true)))
  (`self.SetLifeSpan` _returnvalue 0.05))

(fn `UserConstructionScript`
  (`parent.UserConstructionScript`))