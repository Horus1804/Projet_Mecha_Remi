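; BP_Child_M98B is an M98B weapon child Blueprint that handles firing, reloading and a reversible split animation.
; Fire spends ammo on an object line trace from the barrel socket, with persistent debug drawing, and sends hit zone and damage through BPI_Shoot, using huge damage when InstaKill is set.
; Reload instantly refills ammo to the maximum.
; Split and ReSplit play the ActorSequence forward and in reverse.
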(event `self.ReceiveBeginPlay`
  (`parent.ReceiveBeginPlay`))

(event `self.Split`
  (`ActorSequenceComponent.PlaySequence` (`self.ActorSequence`)))

(event `self.ReSplit`
  (`MovieSceneSequencePlayer.PlayReverse` (`ActorSequenceComponent.SequencePlayer` (`self.ActorSequence`))))

(event `self.Fire`
  (bind _m98b_base (`self.m98b_base`))
  (bind _returnvalue (`SceneComponent.GetSocketLocation` _m98b_base "BarrelEndSocket"))
  (if (!= (`self.actualAmmo`) 0)
    (bind _outhit (`KismetSystemLibrary.LineTraceSingleForObjects` _returnvalue (+ _returnvalue (* (`KismetMathLibrary.GetForwardVector` (`SceneComponent.GetSocketRotation` _m98b_base "BarrelEndSocket")) 1600.0)) (`|MakeArray` "ObjectTypeQuery3" "ObjectTypeQuery2" "ObjectTypeQuery4" :!type "EObjectTypeQuery Enum") false (`|MakeArray` (`GameplayStatics.GetPlayerPawn` 0) :!type "Actor Object Reference") "Persistent"))
    (`/Engine/EditorBlueprintResources/StandardMacros.DecrementInt` (`self.actualAmmo`)
      (:`  `
        (bind (_bblockinghit _binitialoverlap _time _distance _location _impactpoint _normal _impactnormal _physmat _hitactor) (`GameplayStatics.BreakHitResult` _outhit))
        (if (`KismetSystemLibrary.DoesImplementInterface` _hitactor "/Game/Weapon/BPI_Shoot.BPI_Shoot_C")
          (message `/Game/Weapon/BPI_Shoot.ShootHit` _hitactor _physmat _impactpoint self (select `bool` (`self.InstaKill`) :`false` (`self.damage`) :`true` 99999.0)))))))

(event `self.Reload`
  (set `self.actualAmmo` (`self.maxAmmo`)))

(fn `UserConstructionScript`
  (`parent.UserConstructionScript`))