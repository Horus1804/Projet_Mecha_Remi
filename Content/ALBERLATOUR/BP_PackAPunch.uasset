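; BP_PackAPunch is an interactable weapon upgrade station, in the style of a Pack-a-Punch machine.
; Interact checks the player's money against the level-based cost from the weapon's data asset, attaches the weapon to the station, disables firing and calls Split and Upgrade.
; Timed steps then call ReSplit, re-equip the weapon and restore firing.
; AffUi and StopUi toggle a cost widget created at BeginPlay, colored by affordability.
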(event `/Game/BlueprintCommun/BPI_Interact.Interact`
  (params (PlayerRef :type "/Game/Assets/Blueprint/Player/BP_Player Object Reference"))
  (bind _weapontoupgrade (`self.WeaponToUpgrade`))
  (bind _output_get (set `self.Player Ref` PlayerRef))
  (bind _output (`/Game/Assets/Blueprint/Player/BP_Player.Get Current Weapons` _output_get))
  (`/Engine/EditorBlueprintResources/StandardMacros.IsValid` _output
    (:`Is Valid`
      (bind _output_get_2 (set `self.WeaponToUpgrade` _output))
      (if (and (>= (`/Game/Assets/Blueprint/Player/BP_Player.GetMoney` (`self.Player Ref`)) (`BlueprintMapLibrary.Map_Find` (`/Game/Weapon/Blueprint/Data/PDA_Weapon.Cost` (`/Game/Weapon/Blueprint/BP_WeaponParent.DA_Stats` _output_get_2)) (`/Game/Weapon/Blueprint/BP_WeaponParent.LevelGlobalWeapon` _output_get_2))) (not (`/Game/Weapon/Blueprint/BP_WeaponParent.IsOnPackAPunch` _output_get_2)))
        (`/Game/Weapon/Blueprint/BP_WeaponParent.SetOnPackAPunch` _output_get_2 true)
        (`self.K2_DetachFromActor` (`self.WeaponToUpgrade`) "KeepRelative" "KeepRelative" "KeepRelative")
        (`self.K2_AttachToComponent` (`self.WeaponToUpgrade`) (`self.Scene`) "None" "SnapToTarget" "SnapToTarget" "KeepRelative" true)
        (`PrimitiveComponent.SetCollisionResponseToChannel` (`/Game/Weapon/Blueprint/BP_WeaponParent.Box` (`self.WeaponToUpgrade`)) "ECC_GameTraceChannel1" "ECR_Ignore")
        ;[1 1 1] Comment
        (`/Game/Assets/Blueprint/Player/BP_Player.SetCanFire` (`self.Player Ref`) false)
        (`/Game/Weapon/Blueprint/BP_WeaponParent.Split` (`self.WeaponToUpgrade`))
        (`/Engine/EditorBlueprintResources/StandardMacros.IsValid` _weapontoupgrade
          (:`Is Valid`
            (`/Game/Weapon/Blueprint/BP_WeaponParent.Upgrade` _weapontoupgrade "NewEnumerator4")
            (`KismetSystemLibrary.K2_SetTimerDelegate` (delegate `Finish upgrade`) 2.0))
          (:`Is Not Valid`
            (`KismetSystemLibrary.PrintString` "UpgradeNotValid")))))))

(event `Finish upgrade`
  (bind _weapontoupgrade (`self.WeaponToUpgrade`))
  (bind _weapontoupgrade_2 (`self.WeaponToUpgrade`))
  (`/Engine/EditorBlueprintResources/StandardMacros.IsValid` _weapontoupgrade_2
    (:`Is Valid`
      (`PrimitiveComponent.SetCollisionResponseToChannel` (`/Game/Weapon/Blueprint/BP_WeaponParent.Box` _weapontoupgrade_2) "ECC_GameTraceChannel1" "ECR_Block")
      (`/Game/Weapon/Blueprint/BP_WeaponParent.ReSplit` _weapontoupgrade)
      (`KismetSystemLibrary.Delay` 2.0)
      (`/Game/Weapon/Blueprint/BP_WeaponParent.SetOnPackAPunch` _weapontoupgrade false)
      (`/Game/Assets/Blueprint/Player/BP_Player.Equipe Weapon` (`self.Player Ref`) _weapontoupgrade)
      (`/Game/Assets/Blueprint/Player/BP_Player.SetCanFire` (`self.Player Ref`) true))))

(event `self.ReceiveBeginPlay`
  (bind _returnvalue (`|CreateWidget` "/Game/ALBERLATOUR/WBP_PackAPunch.WBP_PackAPunch_C"))
  (bind _output_get (set `self.WBP_PackApunchRef` _returnvalue))
  (`UserWidget.AddToViewport` _output_get 0)
  (`Widget.SetVisibility` _output_get "Hidden"))

(event `/Game/BATET/Bp_buyitem/BPI_AffUI.AffUi`
  (params (PlayerRef :type "/Game/Assets/Blueprint/Player/BP_Player Object Reference"))
  (bind _wbp_packapunchref (`self.WBP_PackApunchRef`))
  (bind _wbp_packapunchref_2 (`self.WBP_PackApunchRef`))
  (`/Engine/EditorBlueprintResources/StandardMacros.IsValid` _wbp_packapunchref
    (:`Is Valid`
      (bind _output (`/Game/Assets/Blueprint/Player/BP_Player.Get Current Weapons` PlayerRef))
      (`/Engine/EditorBlueprintResources/StandardMacros.IsValid` _output
        (:`Is Valid`
          (`Widget.SetVisibility` _wbp_packapunchref "Visible")
          (bind (_value _returnvalue) (`BlueprintMapLibrary.Map_Find` (`/Game/Weapon/Blueprint/Data/PDA_Weapon.Cost` (`/Game/Weapon/Blueprint/BP_WeaponParent.DA_Stats` _output)) (`/Game/Weapon/Blueprint/BP_WeaponParent.LevelGlobalWeapon` _output)))
          (if _returnvalue
            (`/Game/ALBERLATOUR/WBP_PackAPunch.SetCost` _wbp_packapunchref (`KismetTextLibrary.Conv_IntToText` _value))
            (`/Engine/EditorBlueprintResources/StandardMacros.IsValid` _wbp_packapunchref_2
              (:`Is Valid`
                (`/Game/ALBERLATOUR/WBP_PackAPunch.SetColor` _wbp_packapunchref_2 (select `bool` (<= (`/Game/Assets/Blueprint/Player/BP_Player.GetMoney` PlayerRef) _value) :`false` (make `SlateColor` (struct :`R` 0.552941 :`G` 1.0 :`A` 1.0)) :`true` (make `SlateColor` (struct :`R` 1.0 :`A` 1.0))))))))))))

(event `/Game/BATET/Bp_buyitem/BPI_AffUI.StopUi`
  (params (PlayerRef :type "/Game/Assets/Blueprint/Player/BP_Player Object Reference"))
  (bind _wbp_packapunchref (`self.WBP_PackApunchRef`))
  (`/Engine/EditorBlueprintResources/StandardMacros.IsValid` _wbp_packapunchref
    (:`Is Valid`
      (`Widget.SetVisibility` _wbp_packapunchref "Hidden"))))

(fn `UserConstructionScript`)