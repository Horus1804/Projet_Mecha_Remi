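; BP_Nuke is an item-drop pickup that wipes out every zombie when a player touches it.
; Tick spins its static mesh at a configurable rotation speed.
; On overlap with BP_Player it destroys itself, gathers every BP_ZombieMaster actor, then spawns an explosion emitter at each one and calls ExplodeZombie on it.
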(event `self.ReceiveTick`
  (params (DeltaSeconds :type "Float (single-precision)"))
  (`SceneComponent.K2_AddLocalRotation` (`self.StaticMesh`) (`KismetMathLibrary.MakeRotator` 0.0 0.0 (* DeltaSeconds (`self.RotationSpeed`))) false false))

(event `self.StaticMesh.OnComponentBeginOverlap`
  (params (OverlappedComponent :type "PrimitiveComponent Object Reference") (OtherActor :type "Actor Object Reference") (OtherComp :type "PrimitiveComponent Object Reference") (OtherBodyIndex :type Integer) (bFromSweep :type Boolean) (SweepResult :type "HitResult Structure (by ref)"))
  (cast `/Game/Assets/Blueprint/Player/BP_Player` OtherActor)
  (`self.K2_DestroyActor`)
  (bind _outactors (`GameplayStatics.GetAllActorsOfClass` "/Game/Broquere/Zombie/Master/BP_ZombieMaster.BP_ZombieMaster_C"))
  (`KismetSystemLibrary.PrintString` "KABOOOOOOM")
  (for _array_element _outactors
    (`GameplayStatics.SpawnEmitterAtLocation` "/Game/CROUZIE/FXVarietyPack/Particles/P_ky_explosion.P_ky_explosion" (`self.K2_GetActorLocation` _array_element))
    (`/Game/Broquere/Zombie/Master/BP_ZombieMaster.ExplodeZombie` _array_element)))

(fn `UserConstructionScript`)