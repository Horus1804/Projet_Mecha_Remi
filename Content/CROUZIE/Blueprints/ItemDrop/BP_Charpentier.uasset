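; BP_Charpentier is a "carpenter" item drop that instantly rebuilds every barricade when the player touches it.
; The mesh rotates each tick at RotationSpeed until a component hit from BP_Player triggers the pickup.
; It then hides the mesh and disables its collision, calls InstantRebuild on all BP_Barricade actors, prints a debug string, spawns a hit particle effect and destroys itself.
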(event `self.ReceiveTick`
  (params (DeltaSeconds :type "Float (single-precision)"))
  (`SceneComponent.K2_AddLocalRotation` (`self.StaticMesh`) (`KismetMathLibrary.MakeRotator` (* DeltaSeconds (`self.RotationSpeed`))) false false))

(event `self.StaticMesh.OnComponentHit`
  (params (HitComponent :type "PrimitiveComponent Object Reference") (OtherActor :type "Actor Object Reference") (OtherComp :type "PrimitiveComponent Object Reference") (NormalImpulse :type "Vector Structure") (Hit :type "HitResult Structure (by ref)"))
  (cast `/Game/Assets/Blueprint/Player/BP_Player` OtherActor)
  (`self.DisableMesh`)
  (`self.GetAllBarricade`)
  (`KismetSystemLibrary.PrintString` "Ici on charpente ou quoi laaa")
  (`GameplayStatics.SpawnEmitterAtLocation` "/Game/CROUZIE/FXVarietyPack/Particles/P_ky_waterBallHit.P_ky_waterBallHit" (`self.K2_GetActorLocation`) (struct) (0.4 0.4 0.4))
  (`self.K2_DestroyActor`))

(event `DisableMesh`
  (bind _staticmesh (`self.StaticMesh`))
  (`SceneComponent.SetHiddenInGame` _staticmesh true false)
  (`PrimitiveComponent.SetCollisionResponseToAllChannels` _staticmesh "ECR_Ignore")
  (`PrimitiveComponent.SetCollisionEnabled` _staticmesh "NoCollision"))

(event `GetAllBarricade`
  (bind _outactors (`GameplayStatics.GetAllActorsOfClass` "/Game/MathisDENAMUR/BP_Barricade.BP_Barricade_C"))
  (for _array_element _outactors
    (`/Game/MathisDENAMUR/BP_Barricade.InstantRebuild` _array_element)))

(fn `UserConstructionScript`)