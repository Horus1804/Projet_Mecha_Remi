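; BP_Braderie is a rotating item-drop pickup that halves the referenced mystery box's MysteryMoney value, acting as a sale bonus.
; Tick spins the mesh, and a hit from BP_Player destroys the pickup, spawns a water-ball particle burst and halves the value.
; A following 15-second delay is issued on the destroyed actor and leads only to a self-assignment, so the original value is never restored.
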(event `self.ReceiveBeginPlay`)

(event `self.ReceiveTick`
  (params (DeltaSeconds :type "Float (single-precision)"))
  (`SceneComponent.K2_AddLocalRotation` (`self.StaticMesh`) (`KismetMathLibrary.MakeRotator` (* DeltaSeconds (`self.RotationSpeed`))) false false))

(event `self.StaticMesh.OnComponentHit`
  (params (HitComponent :type "PrimitiveComponent Object Reference") (OtherActor :type "Actor Object Reference") (OtherComp :type "PrimitiveComponent Object Reference") (NormalImpulse :type "Vector Structure") (Hit :type "HitResult Structure (by ref)"))
  (bind _mysteryboxeref (`self.MysteryBoxeRef`))
  (cast `/Game/Assets/Blueprint/Player/BP_Player` OtherActor)
  (`self.K2_DestroyActor`)
  (`/Engine/EditorBlueprintResources/StandardMacros.IsValid` _mysteryboxeref
    (:`Is Valid`
      (`GameplayStatics.SpawnEmitterAtLocation` "/Game/CROUZIE/FXVarietyPack/Particles/P_ky_waterBallHit.P_ky_waterBallHit" (`self.K2_GetActorLocation`) (struct) (0.4 0.4 0.4))
      (set `/Game/Julien/MysteryBox/BP_Mystery_Box.MysteryMoney` (/ (`/Game/Julien/MysteryBox/BP_Mystery_Box.MysteryMoney` _mysteryboxeref) 2) _mysteryboxeref)
      (`KismetSystemLibrary.Delay` 15.0)
      (set `/Game/Julien/MysteryBox/BP_Mystery_Box.MysteryMoney` (`/Game/Julien/MysteryBox/BP_Mystery_Box.MysteryMoney` _mysteryboxeref) _mysteryboxeref))))

(fn `UserConstructionScript`)