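; BP_Skull is an insta-kill pickup, shown as a skull item that spins its mesh every tick.
; When BP_Player hits the mesh and holds a valid weapon, it hides itself, disables collision and spawns a burst effect.
; It sets InstaKill on that current weapon, then clears it after a 15-second delay.
; The actor stays alive but hidden, as its DestroyActor call is unconnected.
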(event `self.ReceiveTick`
  (params (DeltaSeconds :type "Float (single-precision)"))
  (`SceneComponent.K2_AddLocalRotation` (`self.StaticMesh`) (`KismetMathLibrary.MakeRotator` 0.0 (* DeltaSeconds (`self.RotationSpeed`))) false false))

(event `self.StaticMesh.OnComponentHit`
  (params (HitComponent :type "PrimitiveComponent Object Reference") (OtherActor :type "Actor Object Reference") (OtherComp :type "PrimitiveComponent Object Reference") (NormalImpulse :type "Vector Structure") (Hit :type "HitResult Structure (by ref)"))
  (bind _asbp_player (cast `/Game/Assets/Blueprint/Player/BP_Player` OtherActor))
  (bind _output (`/Game/Assets/Blueprint/Player/BP_Player.Get Current Weapons` _asbp_player))
  (`/Engine/EditorBlueprintResources/StandardMacros.IsValid` _output
    (:`Is Valid`
      (`self.Disabled`)
      (`GameplayStatics.SpawnEmitterAtLocation` "/Game/CROUZIE/FXVarietyPack/Particles/P_ky_waterBallHit.P_ky_waterBallHit" (`self.K2_GetActorLocation`) (struct) (0.4 0.4 0.4))
      (set `/Game/Weapon/Blueprint/BP_WeaponParent.InstaKill` true _output)
      (`KismetSystemLibrary.Delay` 15.0)
      (set `/Game/Weapon/Blueprint/BP_WeaponParent.InstaKill` false _output))))

(event `Disabled`
  (`SceneComponent.SetHiddenInGame` (`self.StaticMesh`) true false)
  (`PrimitiveComponent.SetCollisionEnabled` (`self.StaticMesh`) "NoCollision")
  (`SceneComponent.SetHiddenInGame` (`self.ParticleSystem`) true false))

(fn `UserConstructionScript`)