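; BP_MaxAmmo is a spinning max-ammo pickup that refills the player's weapons on contact.
; Tick rotates the static mesh in yaw at RotationSpeed, and BeginPlay caches a reference to player 0's BP_Player.
; When the mesh is hit by a BP_Player, the actor destroys itself, prints a debug message and sets every WeaponsSlot entry's ammo to its maximum.
; A water-hit particle effect spawns at the pickup's location once per refilled weapon.
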(event `self.ReceiveBeginPlay`
  (bind _asbp_player (cast `/Game/Assets/Blueprint/Player/BP_Player` (`GameplayStatics.GetPlayerCharacter` 0)))
  (set `self.PLayerRef` _asbp_player))

(event `self.ReceiveTick`
  (params (DeltaSeconds :type "Float (single-precision)"))
  (`SceneComponent.K2_AddLocalRotation` (`self.StaticMesh`) (`KismetMathLibrary.MakeRotator` 0.0 0.0 (* DeltaSeconds (`self.RotationSpeed`))) false false))

(event `self.StaticMesh.OnComponentHit`
  (params (HitComponent :type "PrimitiveComponent Object Reference") (OtherActor :type "Actor Object Reference") (OtherComp :type "PrimitiveComponent Object Reference") (NormalImpulse :type "Vector Structure") (Hit :type "HitResult Structure (by ref)"))
  (cast `/Game/Assets/Blueprint/Player/BP_Player` OtherActor)
  (`self.K2_DestroyActor`)
  (`KismetSystemLibrary.PrintString` "Pleins de munitions la OUIIII")
  (for _array_element (`/Game/Assets/Blueprint/Player/BP_Player.WeaponsSlot` (`self.PLayerRef`))
    (set `/Game/Weapon/Blueprint/BP_WeaponParent.actualAmmo` (`/Game/Weapon/Blueprint/BP_WeaponParent.maxAmmo` _array_element) _array_element)
    (`GameplayStatics.SpawnEmitterAtLocation` "/Game/CROUZIE/FXVarietyPack/Particles/P_ky_waterBallHit.P_ky_waterBallHit" (`self.K2_GetActorLocation`) (struct) (0.4 0.4 0.4))))

(fn `UserConstructionScript`)