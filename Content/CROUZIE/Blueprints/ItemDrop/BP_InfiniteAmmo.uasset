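; BP_InfiniteAmmo is a rotating power-up pickup that gives BP_Player temporary infinite ammo.
; On mesh hit by the player, it hides itself, disables collision, spawns a particle burst and saves each weapon slot's MaxAmmo.
; It fakes infinity with a huge ActualAmmo and starts a 12-second timer.
; RemoveInfiniteAmmo sets max and current ammo to the saved maximum, leaving weapons full, refreshes the UI and destroys the actor.
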(event `self.ReceiveTick`
  (params (DeltaSeconds :type "Float (single-precision)"))
  (`SceneComponent.K2_AddLocalRotation` (`self.StaticMesh`) (`KismetMathLibrary.MakeRotator` 0.0 (* DeltaSeconds (`self.RotationSpeed`))) false false))

(event `self.StaticMesh.OnComponentHit`
  (params (HitComponent :type "PrimitiveComponent Object Reference") (OtherActor :type "Actor Object Reference") (OtherComp :type "PrimitiveComponent Object Reference") (NormalImpulse :type "Vector Structure") (Hit :type "HitResult Structure (by ref)"))
  (bind _asbp_player (cast `/Game/Assets/Blueprint/Player/BP_Player` OtherActor))
  (set `self.As BP Player` _asbp_player)
  (`self.DisablePowerUps`)
  (`KismetSystemLibrary.PrintString` "Pleins de munitions la OUIIII")
  (`self.GetActualAmmo`)
  (`GameplayStatics.SpawnEmitterAtLocation` "/Game/CROUZIE/FXVarietyPack/Particles/P_ky_waterBallHit.P_ky_waterBallHit" (`self.K2_GetActorLocation`) (struct) (0.4 0.4 0.4))
  (`self.SetInfiniteAmmo`)
  (`KismetSystemLibrary.K2_SetTimerDelegate` (`|CreateDelegate` :!event `RemoveInfiniteAmmo`) 12.0))

(event `DisablePowerUps`
  (bind _staticmesh (`self.StaticMesh`))
  ;[1 0.04246 0.988] Disable Power Up
  (`SceneComponent.SetHiddenInGame` _staticmesh true false)
  (`PrimitiveComponent.SetCollisionResponseToAllChannels` _staticmesh "ECR_Ignore")
  (`PrimitiveComponent.SetCollisionEnabled` _staticmesh "NoCollision"))

(event `GetActualAmmo`
  ;[0.04999 0.03478 1] Get Actual Ammo
  (for _array_element (`/Game/Assets/Blueprint/Player/BP_Player.WeaponsSlot` (`self.As BP Player`))
    (`KismetArrayLibrary.Array_Add` (`self.SaveAmmo`) (`/Game/Weapon/Blueprint/BP_WeaponParent.maxAmmo` _array_element))))

(event `SetInfiniteAmmo`
  (bind _as_bp_player (`self.As BP Player`))
  ;[0.2083 0 1] Infinite Ammo
  (for _array_element (`/Game/Assets/Blueprint/Player/BP_Player.WeaponsSlot` _as_bp_player)
    (set `/Game/Weapon/Blueprint/BP_WeaponParent.actualAmmo` 99999999 _array_element))
  (`/Game/Assets/Blueprint/Player/BP_Player.UpdateReloadUI` _as_bp_player))

(event `RemoveInfiniteAmmo`
  (bind _saveammo (`self.SaveAmmo`))
  (bind _as_bp_player (`self.As BP Player`))
  ;[1 0.8557 0] Remove Infinite Ammo
  (for (_array_element _array_index) (`/Game/Assets/Blueprint/Player/BP_Player.WeaponsSlot` _as_bp_player)
    (if (`KismetArrayLibrary.Array_IsValidIndex` _saveammo _array_index)
      (bind _output (`|GetArrayItem` _saveammo _array_index))
      (set `/Game/Weapon/Blueprint/BP_WeaponParent.maxAmmo` _output _array_element)
      (set `/Game/Weapon/Blueprint/BP_WeaponParent.actualAmmo` _output _array_element)))
  (`/Game/Assets/Blueprint/Player/BP_Player.UpdateReloadUI` _as_bp_player)
  (`self.K2_DestroyActor`))

(fn `UserConstructionScript`)