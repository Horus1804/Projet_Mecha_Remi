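; Master zombie enemy character for a wave-based shooter, with randomized modular outfit meshes, materials and morphs, and walk or run speed set on possession.
; Socket sphere traces deal melee damage for each arm and head.
; Weapon hits scale damage, score and money by hit zone, with weapon and distance modifiers.
; Death ragdolls the body, credits kills and may drop power-ups, while a timer kills zombies that stay too slow.
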(event `self.ReceivePossessed`
  (params (NewController :type "Controller Object Reference"))
  ;[0.1946 0.009721 0.009134] Event Possessed
  (bind _asaic_zombie (cast `/Game/Broquere/AI/AIC_Zombie` NewController))
  (set `self.RefAIC Zombie` _asaic_zombie)
  (`self.IsRunningZombi`))

(event `IsRunningZombi`
  (bind _charactermovement (`self.CharacterMovement`))
  ;[0 0.2697 1] Set Zombie Can Running
  (if (`self.IsRunning`)
    (set `CharacterMovementComponent.MaxWalkSpeed` 280.0 _charactermovement)
    (else
      (set `CharacterMovementComponent.MaxWalkSpeed` 45.0 _charactermovement))))

(event `self.ReceiveBeginPlay`
  ;[0.1329 0.03689 0.0356] Event BeginPlay
  (bind _returnvalue (`KismetSystemLibrary.K2_SetTimer` null "ZombieCantStayInPlace" 1.0 true))
  (set `self.Event_ZombieCantStayInPlace` _returnvalue)
  (bind _output_get (set `self.As BPC Outfit Controller` (`self.GetComponentByClass` "/Game/Broquere/Zombie/Master/BPC_OutfitController_Testing.BPC_OutfitController_Testing_C")))
  (`/Game/Broquere/Zombie/Master/BPC_OutfitController_Testing.RandomizeSelected` _output_get null)
  (bind _output_get_2 (set `self.As BPC Outfit Controller` (`self.GetComponentByClass` "/Game/Broquere/Zombie/Master/BPC_OutfitController_Testing.BPC_OutfitController_Testing_C")))
  (`/Engine/EditorBlueprintResources/StandardMacros.IsValid` _output_get_2
    (:`Is Valid`
      (if (`/Game/Broquere/Zombie/Master/BPC_OutfitController_Testing.RandomizeOnBeginPlay` _output_get_2)
        (`/Game/Broquere/Zombie/Master/BPC_OutfitController_Testing.RandomizeSelected` _output_get_2 self)))))

(event `SetComponentArrays`
  (bind _countright (`self.countRight`))
  (bind _countleft (`self.countLeft`))
  ;[0.4639 1 0.4455] Construct Body of Zombie
  (`KismetArrayLibrary.Array_Clear` (`self.SkeletalMesh`))
  (`KismetArrayLibrary.Array_Clear` (`self.StaticMesh`))
  (`|ExecutionSequence`
    (:`then_0`
      (bind _output_get (set `self.SkeletalMesh` (`self.GetComponentsByTag` "/Script/Engine.SkeletalMeshComponent" "OutfitController")))
      (for _array_element _output_get
        (`PrimitiveComponent.SetCollisionObjectType` _array_element "ECC_Pawn")
        (`PrimitiveComponent.SetCollisionEnabled` _array_element "QueryAndPhysics")
        (`|ExecutionSequence`
          (:`then_0`
            (bind _returnvalue (`KismetSystemLibrary.GetDisplayName` _array_element))
            (if (`KismetStringLibrary.Contains` _returnvalue "ArmLeft" true)
              (if (> _countleft 10)
                (set `self.HasLeftArm` true)
                (else
                  (`/Engine/EditorBlueprintResources/StandardMacros.IncrementInt` _countleft)))))
          (:`then_1`
            (if (`KismetStringLibrary.Contains` _returnvalue "ArmRight" true)
              (if (> _countright 10)
                (set `self.HasRightArm` true)
                (else
                  (`/Engine/EditorBlueprintResources/StandardMacros.IncrementInt` _countright))))))))
    (:`then_1`
      (set `self.StaticMesh` (`self.GetComponentsByTag` "/Script/Engine.StaticMeshComponent" "OutfitController")))))

(event `ClearComponents`
  ;[1 0 0.9305] Clear Components Body
  (`self.SetComponentArrays`)
  (`|ExecutionSequence`
    (:`then_0`
      (for _array_element (`self.SkeletalMesh`)
        (if (`ActorComponent.ComponentHasTag` _array_element "UE5Master")
          _
          (elif (`ActorComponent.ComponentHasTag` _array_element "Parent")
            (`SkinnedMeshComponent.SetSkinnedAssetAndUpdate` _array_element null true)
            (else
              (`ActorComponent.K2_DestroyComponent` _array_element))))))
    (:`then_1`
      (for _array_element_2 (`self.StaticMesh`)
        (`ActorComponent.K2_DestroyComponent` _array_element_2)))))

(event `SetMaterials`
  (params (SlotNames :type "Array of String") (ParameterNames :type "Array of String") (Materials :type "Array of MaterialInstance Object Reference") (ParameterValue :type "Float (double-precision)") (RandomizeParameters :type Boolean))
  (bind _skeletalmesh (`self.SkeletalMesh`))
  ;[0 0.9179 1] Set Materials for Zombie
  (`self.SetComponentArrays`)
  (if RandomizeParameters
    (for (_array_element _array_index) Materials
      (bind _returnvalue (`KismetMaterialLibrary.CreateDynamicMaterialInstance` _array_element "None" "Transient"))
      (for _array_element_2 ParameterNames
        (`/Engine/EditorBlueprintResources/StandardMacros.IsValid` _returnvalue
          (:`Is Valid`
            (`MaterialInstanceDynamic.SetScalarParameterValue` _returnvalue (`KismetStringLibrary.Conv_StringToName` _array_element_2) ParameterValue))))
      (for _array_element_3 _skeletalmesh
        (bind _output (`|GetArrayItem` SlotNames _array_index))
        (`PrimitiveComponent.SetMaterialByName` _array_element_3 (`KismetStringLibrary.Conv_StringToName` _output) _returnvalue)))
    (else
      (for (_array_element_4 _array_index_2) SlotNames
        (`|ExecutionSequence`
          (:`then_0`
            (for _array_element_5 _skeletalmesh
              (`PrimitiveComponent.SetMaterialByName` _array_element_5 (`KismetStringLibrary.Conv_StringToName` (select `bool` RandomizeParameters :`false` _array_element_4 :`true` _output)) (select `bool` RandomizeParameters :`false` (`|GetArrayItem` Materials _array_index_2) :`true` _returnvalue :!type "MaterialInterface Object Reference")))))))))

(event `SetMorphTarget`
  (params (RandomValues :type "Float (double-precision)"))
  ;[0.9134 1 0] Set Morhping target for Face
  (`self.SetComponentArrays`)
  (for _array_element (`self.SkeletalMesh`)
    (for _array_element_2 (`/Game/Broquere/Zombie/Master/BPC_OutfitController_Testing.MorphTargets` (`self.As BPC Outfit Controller`))
      (for _array_element_3 (`.MorphposeName_4_6D07119D4EF681519045DBA1FD4884E3` (break `/Game/YI_ModularZombies/Blueprints/Master/Data/Struc_StaticMorphPoses` _array_element_2))
        (`SkeletalMeshComponent.SetMorphTarget` _array_element (`KismetStringLibrary.Conv_StringToName` _array_element_3) RandomValues true)))))

(event `Attack_Zombi_LeftHand`
  (bind _parent (`self.Parent`))
  ;[1 0 0.02652] Zombi Attack Damage
  ;;[1 0 0.8233] Left Arm
  (if (not (`self.IsDead`))
    (if (`self.HasLeftArm`)
      (bind (_outhit _returnvalue) (`KismetSystemLibrary.SphereTraceSingle` :`Start` (`SceneComponent.GetSocketLocation` _parent "AtkStartLSocket") :`End` (`SceneComponent.GetSocketLocation` _parent "AtkEndLSocket") :`Radius` 20.0 :`TraceChannel` "TraceTypeQuery1" :`DrawDebugType` "ForOneFrame"))
      (if _returnvalue
        (bind (_bblockinghit _binitialoverlap _time _distance _location _impactpoint _normal _impactnormal _physmat _hitactor) (`GameplayStatics.BreakHitResult` _outhit))
        (cast `/Game/Broquere/Zombie/Master/BP_ZombieMaster` _hitactor
          (:`CastFailed`
            (`/Engine/EditorBlueprintResources/StandardMacros.DoOnce` false :!label _label
              (:`Completed`
                (`GameplayStatics.ApplyDamage` _hitactor 10.0 null self)))))
        (else
          (goto _label :!via `Reset`)))
      (elif (not (`self.HasRightArm`))
        (`self.AttackZombi_Head`)))))

(event `ResetAttackArmLeft`
  ;[1 0 0.02652] Zombi Attack Damage
  ;;[1 0 0.8233] Left Arm
  (goto _label :!via `Reset`))

(event `Attack_Zombi_RightHand`
  (bind _parent (`self.Parent`))
  ;[1 0 0.02652] Zombi Attack Damage
  ;;[1 0.7728 0] Right Arm
  (if (not (`self.IsDead`))
    (if (`self.HasRightArm`)
      (bind (_outhit _returnvalue) (`KismetSystemLibrary.SphereTraceSingle` :`Start` (`SceneComponent.GetSocketLocation` _parent "AtkStartRSocket") :`End` (`SceneComponent.GetSocketLocation` _parent "AtkEndRSocket") :`Radius` 20.0 :`TraceChannel` "TraceTypeQuery1" :`DrawDebugType` "ForOneFrame"))
      (if _returnvalue
        (bind (_bblockinghit _binitialoverlap _time _distance _location _impactpoint _normal _impactnormal _physmat _hitactor) (`GameplayStatics.BreakHitResult` _outhit))
        (cast `/Game/Broquere/Zombie/Master/BP_ZombieMaster` _hitactor
          (:`CastFailed`
            (`/Engine/EditorBlueprintResources/StandardMacros.DoOnce` false :!label _label_2
              (:`Completed`
                (`GameplayStatics.ApplyDamage` _hitactor 10.0 null self)))))
        (else
          (goto _label_2 :!via `Reset`))))))

(event `Reset attack Arm Right`
  ;[1 0 0.02652] Zombi Attack Damage
  ;;[1 0.7728 0] Right Arm
  (goto _label_2 :!via `Reset`))

(event `AttackZombi_Head`
  (bind _parent (`self.Parent`))
  ;[1 0 0.02652] Zombi Attack Damage
  ;;[0 1 0.1175] Head
  (if (not (`self.IsDead`))
    (bind (_outhit _returnvalue) (`KismetSystemLibrary.SphereTraceSingle` :`Start` (`SceneComponent.GetSocketLocation` _parent "neck_01Socket") :`End` (`SceneComponent.GetSocketLocation` _parent "headSocket") :`Radius` 20.0 :`TraceChannel` "TraceTypeQuery1" :`DrawDebugType` "ForOneFrame"))
    (if _returnvalue
      (bind (_bblockinghit _binitialoverlap _time _distance _location _impactpoint _normal _impactnormal _physmat _hitactor) (`GameplayStatics.BreakHitResult` _outhit))
      (cast `/Game/Broquere/Zombie/Master/BP_ZombieMaster` _hitactor
        (:`CastFailed`
          (`/Engine/EditorBlueprintResources/StandardMacros.DoOnce` false :!label _label_3
            (:`Completed`
              (`GameplayStatics.ApplyDamage` _hitactor 10.0 null self)))))
      (else
        (goto _label_3 :!via `Reset`)))))

(event `Reset AttackHead`
  ;[1 0 0.02652] Zombi Attack Damage
  ;;[0 1 0.1175] Head
  (goto _label_3 :!via `Reset`))

(event `DisableCollisionMeshPart`
  (bind _staticmesh (`self.StaticMesh`))
  (bind _skeletalmesh (`self.SkeletalMesh`))
  ;[0.8955 1 0] Permet de réinitialiser les collisions de chaque partie de membres du zombie
  (if (`KismetArrayLibrary.Array_IsNotEmpty` _staticmesh)
    (for _array_element _staticmesh
      (`PrimitiveComponent.SetCollisionObjectType` _array_element "ECC_PhysicsBody")
      (`PrimitiveComponent.SetCollisionResponseToAllChannels` _array_element "ECR_Ignore")
      (`PrimitiveComponent.SetCollisionEnabled` _array_element "NoCollision")))
  (if (`KismetArrayLibrary.Array_IsNotEmpty` _skeletalmesh)
    (for _array_element_2 _skeletalmesh
      (`PrimitiveComponent.SetCollisionObjectType` _array_element_2 "ECC_PhysicsBody")
      (`PrimitiveComponent.SetCollisionResponseToAllChannels` _array_element_2 "ECR_Ignore")
      (`PrimitiveComponent.SetCollisionEnabled` _array_element_2 "NoCollision"))))

(event `/Game/Weapon/BPI_Shoot.ShootHit`
  (params (HitZone :type "PhysicalMaterial Object Reference") (HitLocation :type "Vector Structure") (Causer :type "Actor Object Reference") (BaseDamage :type "Float (double-precision)"))
  (bind _asbp_weapon_parent (cast `/Game/Weapon/Blueprint/BP_WeaponParent` Causer :!pure true))
  (bind _surfacetype (`PhysicalMaterial.SurfaceType` HitZone))
  (bind _weapontype (`/Game/Weapon/Blueprint/BP_WeaponParent.WeaponType` _asbp_weapon_parent))
  ;[1 0.09369 0.8863] Permet de prendre des damages via les armes du joueur
  (`GameplayStatics.ApplyDamage` self (+ BaseDamage (select `EPhysicalSurface` _surfacetype :`SurfaceType_Default` 10.0 :`SurfaceType1` 100.0 :`SurfaceType2` 20.0 :`SurfaceType3` 35.0 :`SurfaceType4` 50.0 :!type "Float (single-precision)")) null Causer)
  (`NiagaraFunctionLibrary.SpawnSystemAtLocation` "/Game/YI_BloodDroplets/Particles/GPU/FX_Punch_GPU.FX_Punch_GPU" HitLocation (`self.K2_GetActorRotation` Causer))
  (`GameplayStatics.PlaySoundAtLocation` (select `EPhysicalSurface` _surfacetype :`SurfaceType_Default` "/Game/Assets/Audio/Zombie/Hit/SC_Zombie_Hit_Torse.SC_Zombie_Hit_Torse" :`SurfaceType1` "/Game/Assets/Audio/Zombie/Hit/SC_Zombie_Hit_Head.SC_Zombie_Hit_Head" :`SurfaceType2` "/Game/Assets/Audio/Zombie/Hit/SC_Zombie_Hit_Arm.SC_Zombie_Hit_Arm" :`SurfaceType3` "/Game/Assets/Audio/Zombie/Hit/SC_Zombie_Hit_Leg.SC_Zombie_Hit_Leg" :`SurfaceType4` "/Game/Assets/Audio/Zombie/Hit/SC_Zombie_Hit_Torse.SC_Zombie_Hit_Torse" :!type "SoundBase Object Reference") (`self.K2_GetActorLocation`) (struct) 0.25 1.0 0.0 "/Game/YI_ModularZombies/Sounds/Master/SA_Low.SA_Low" null null null)
  (`self.SetScore` HitZone _asbp_weapon_parent _weapontype)
  (`self.AddMoneyToPlayer` HitZone _weapontype))

(event `self.OnLanded`
  (params (Hit :type "HitResult Structure (by ref)"))
  ;[0.5057 1 0.231] On Landed Sound
  (`GameplayStatics.PlaySoundAtLocation` "/Game/Assets/Audio/Zombie/Jump/SC_Zombie_Land.SC_Zombie_Land" (`self.K2_GetActorLocation`) (struct) 0.3 1.0 0.0 "/Game/YI_ModularZombies/Sounds/Master/SA_Low.SA_Low" null null null)
  (`GameplayStatics.ApplyDamage` self 2.0 null self))

(event `self.ReceiveAnyDamage`
  (params (Damage :type "Float (single-precision)") (DamageType :type "DamageType Object Reference") (InstigatedBy :type "Controller Object Reference") (DamageCauser :type "Actor Object Reference"))
  (bind _playerref (`/Game/Broquere/AI/AIC_Zombie.PlayerRef` (`self.RefAIC Zombie`)))
  ;[0.2962 0 1] Get Any Damage
  (if (not (`self.IsDead`))
    (bind _output_get (set `self.Health` (- (`self.Health`) Damage)))
    (if (<= _output_get 0.0)
      (set `self.IsDead` true)
      (`self.SetDead`)
      (`self.SpawnPowerUps`)
      (`/Engine/EditorBlueprintResources/StandardMacros.IsValid` _playerref
        (:`Is Valid`
          (`/Game/Assets/Blueprint/Player/BP_Player.AddKills` _playerref 1))))))

(event `SetDead`
  (bind _event_zombiecantstayinplace (`self.Event_ZombieCantStayInPlace`))
  (bind _capsulecomponent (`self.CapsuleComponent`))
  (bind _parent (`self.Parent`))
  ;[0.0446 0 1] Setup Body for Death
  (`SkeletalMeshComponent.Stop` (`self.Mesh`))
  (`SkeletalMeshComponent.Stop` (`self.Parent`))
  (`PrimitiveComponent.SetCollisionResponseToAllChannels` _capsulecomponent "ECR_Ignore")
  (`PrimitiveComponent.SetCollisionEnabled` _capsulecomponent "NoCollision")
  (`PrimitiveComponent.SetCollisionResponseToAllChannels` _parent "ECR_Ignore")
  (`PrimitiveComponent.SetCollisionEnabled` _parent "NoCollision")
  (`self.DisableCollisionMeshPart`)
  (`PrimitiveComponent.SetSimulatePhysics` (`self.Mesh`) true)
  (`GameplayStatics.PlaySoundAtLocation` "/Game/Assets/Audio/Zombie/Hit/SC_Zombie_Hit_Head.SC_Zombie_Hit_Head" (`self.K2_GetActorLocation`) (struct) 0.5 1.0 0.0 "/Game/YI_ModularZombies/Sounds/Master/SA_Low.SA_Low" null null null)
  (`KismetSystemLibrary.K2_SetTimerDelegate` (`|CreateDelegate` :!event `DestroyZombie`) 5.0)
  (if (`KismetSystemLibrary.K2_IsTimerActiveHandle` _event_zombiecantstayinplace)
    (`KismetSystemLibrary.K2_ClearAndInvalidateTimerHandle` _event_zombiecantstayinplace)))

(event `DestroyZombie`
  (bind _spawner (`self.Spawner`))
  ;[0.8439 0.386 1] Destroy Zombie
  (`/Engine/EditorBlueprintResources/StandardMacros.IsValid` _spawner
    (:`Is Valid`
      (`/Engine/EditorBlueprintResources/StandardMacros.DecrementInt` (`/Game/Broquere/BP_SpawnZombi.NumberOfZombies` _spawner)
        (:`  `
          (`/Game/Broquere/BP_SpawnZombi.HandleWave` _spawner))))
    (:`Is Not Valid`
      _))
  (`self.K2_DestroyActor`))

(event `ExplodeZombie`
  (bind _event_zombiecantstayinplace (`self.Event_ZombieCantStayInPlace`))
  (bind _playerref (`/Game/Broquere/AI/AIC_Zombie.PlayerRef` (`self.RefAIC Zombie`)))
  ;[1 0 0.1278] Explode Zombie
  (set `self.IsDead` true)
  (`NiagaraFunctionLibrary.SpawnSystemAtLocation` "/Game/YI_BloodDroplets/Particles/GPU/FX_Timed_Bleeding_GPU.FX_Timed_Bleeding_GPU" (`self.K2_GetActorLocation`) (`self.K2_GetActorRotation`))
  (`PrimitiveComponent.SetCollisionResponseToAllChannels` (`self.CapsuleComponent`) "ECR_Ignore")
  (`PrimitiveComponent.SetSimulatePhysics` (`self.Parent`) true)
  (`PrimitiveComponent.SetCollisionResponseToChannel` (`self.Mesh`) "ECC_Pawn" "ECR_Ignore")
  (`PrimitiveComponent.SetCollisionResponseToChannel` (`self.Parent`) "ECC_Pawn" "ECR_Ignore")
  (for _array_element (`self.SkeletalMesh`)
    (`PrimitiveComponent.SetCollisionResponseToChannel` _array_element "ECC_Pawn" "ECR_Ignore")
    (`PrimitiveComponent.SetSimulatePhysics` _array_element true))
  (`/Engine/EditorBlueprintResources/StandardMacros.IsValid` _playerref
    (:`Is Valid`
      (`/Game/Assets/Blueprint/Player/BP_Player.AddKills` _playerref 1)
      (`self.SetScore` "/Game/Weapon/PM_Torso.PM_Torso" _playerref "NewEnumerator5")
      (`self.AddMoneyToPlayer` "/Game/Weapon/PM_Torso.PM_Torso" "NewEnumerator5"))
    (:`Is Not Valid`
      _))
  (`KismetSystemLibrary.K2_SetTimerDelegate` (`|CreateDelegate` :!event `DestroyZombie`) 5.0)
  (if (`KismetSystemLibrary.K2_IsTimerActiveHandle` _event_zombiecantstayinplace)
    (`KismetSystemLibrary.K2_ClearAndInvalidateTimerHandle` _event_zombiecantstayinplace)))

(fn `AddDamage`
  (params (AttackDamage :type "Float (double-precision)"))
  (set `self.AttackDamage` (+ AttackDamage (`self.AttackDamage`))))

(fn `AddHealth`
  (params (Health :type "Float (double-precision)"))
  (locals (LocalHealth :type "Float (double-precision)"))
  (bind _maxhealth (`self.MaxHealth`))
  (bind _output_get (set `local.LocalHealth` (+ Health (`self.Health`))))
  (set `self.Health` (select `bool` (>= _output_get _maxhealth) :`false` _output_get :`true` _maxhealth)))

(fn `AddMaxHealth`
  (params (MaxHealth :type "Float (double-precision)"))
  (set `self.MaxHealth` (+ MaxHealth (`self.MaxHealth`))))

(fn `AddMoneyToPlayer`
  (params (`Hit Zone` :type "PhysicalMaterial Object Reference") (`Weapon Type` :type "/Game/Assets/Blueprint/Player/Enum/EWeaponType Enum" :default "NewEnumerator0"))
  (locals (LocalMoney :type Integer))
  (bind _playerref (`/Game/Broquere/AI/AIC_Zombie.PlayerRef` (`self.RefAIC Zombie`)))
  (`/Engine/EditorBlueprintResources/StandardMacros.IsValid` _playerref
    (:`Is Valid`
      (bind _output_get (set `local.LocalMoney` (+ (select `EPhysicalSurface` (`PhysicalMaterial.SurfaceType` `Hit Zone`) :`SurfaceType_Default` 10 :`SurfaceType1` 100 :`SurfaceType2` 25 :`SurfaceType3` 25 :`SurfaceType4` 30) (select `/Game/Assets/Blueprint/Player/Enum/EWeaponType` `Weapon Type` :`NewEnumerator0` 10 :`NewEnumerator1` 10 :`NewEnumerator2` 15 :`NewEnumerator6` 15 :`NewEnumerator7` 15 :`NewEnumerator8` 15 :`NewEnumerator9` 15 :`NewEnumerator3` 5 :`NewEnumerator4` 20 :`NewEnumerator5` 20))))
      (`/Game/Assets/Blueprint/Player/BP_Player.AddMoney` _playerref _output_get))))

(fn `AddScore`
  (params (Score :type "Float (double-precision)"))
  (set `self.Score` (+ Score (`self.Score`))))

(fn `GetDamage`
  (returns (AttackDamage :type "Float (double-precision)"))
  (return (`self.AttackDamage`)))

(fn `GetHealth`
  (returns (Health :type "Float (double-precision)"))
  (return (`self.Health`)))

(fn `GetIsDead`
  (returns (IsDead :type Boolean))
  (return (`self.IsDead`)))

(fn `GetIsRunning`
  (returns (IsRunning :type Boolean))
  (return (`self.IsRunning`)))

(fn `GetMaxHealth`
  (returns (MaxHealth :type "Float (double-precision)"))
  (return (`self.MaxHealth`)))

(fn `GetScore`
  (returns (Score :type "Float (double-precision)"))
  (return (`self.Score`)))

(fn `ScoreMultiplierByDistance`
  (params (Hitter :type "Actor Object Reference"))
  (returns (Multiplier :type "Float (double-precision)"))
  (bind _returnvalue (`KismetMathLibrary.Vector_Distance` (`self.K2_GetActorLocation` Hitter) (`self.K2_GetActorLocation` self)))
  (if (> _returnvalue 750.0)
    (return 0.75)
    (elif (< _returnvalue 150.0)
      (return 1.25)
      (else
        (return (`KismetMathLibrary.Lerp` 0.75 1.25 (/ (- _returnvalue 150.0) 650.0)))))))

(fn `SetDamage`
  (params (AttackDamage :type "Float (double-precision)"))
  (set `self.AttackDamage` AttackDamage))

(fn `SetHealth`
  (params (Health :type "Float (double-precision)"))
  (bind _maxhealth (`self.MaxHealth`))
  (set `self.Health` (select `bool` (>= Health _maxhealth) :`false` Health :`true` _maxhealth)))

(fn `SetMaxHealth`
  (params (MaxHealth :type "Float (double-precision)"))
  (set `self.MaxHealth` MaxHealth))

(fn `SetScore`
  (params (`Hit Zone` :type "PhysicalMaterial Object Reference") (`Damaged By` :type "Actor Object Reference") (`Weapon Type` :type "/Game/Assets/Blueprint/Player/Enum/EWeaponType Enum" :default "NewEnumerator0"))
  (bind _playerref (`/Game/Broquere/AI/AIC_Zombie.PlayerRef` (`self.RefAIC Zombie`)))
  (bind _output_get (set `self.Score` (* (select `EPhysicalSurface` (`PhysicalMaterial.SurfaceType` `Hit Zone`) :`SurfaceType_Default` 50.0 :`SurfaceType1` 75.0 :`SurfaceType2` 35.0 :`SurfaceType3` 35.0 :`SurfaceType4` 50.0 :!type "Float (single-precision)") (`self.ScoreMultiplierByDistance` `Damaged By`) (select `/Game/Assets/Blueprint/Player/Enum/EWeaponType` `Weapon Type` :`NewEnumerator0` 1.0 :`NewEnumerator1` 1.0 :`NewEnumerator2` 0.95 :`NewEnumerator6` 1.05 :`NewEnumerator7` 1.0 :`NewEnumerator8` 1.1 :`NewEnumerator9` 0.9 :`NewEnumerator3` 0.9 :`NewEnumerator4` 0.95 :`NewEnumerator5` 2.0))))
  (`/Engine/EditorBlueprintResources/StandardMacros.IsValid` _playerref
    (:`Is Valid`
      (`/Game/Assets/Blueprint/Player/BP_Player.Addscore` _playerref (`KismetMathLibrary.Round` _output_get)))))

(fn `SpawnPowerUps`
  (locals (LocalRandom :type Byte))
  (bind _array (`self.GetPowerUpsList`))
  (if (`KismetMathLibrary.RandomBoolWithWeight` 0.02)
    (if (`KismetArrayLibrary.Array_IsNotEmpty` _array)
      (set `local.LocalRandom` (`KismetMathLibrary.Conv_IntToByte` (`KismetMathLibrary.RandomIntegerInRange` 0 (- (`KismetArrayLibrary.Array_Length` _array) 1))))
      (for (_array_element _array_index) _array
        (if (== _array_index (`local.LocalRandom`))
          (`|SpawnActorFromClass` _array_element (`KismetMathLibrary.MakeTransform` (`self.K2_GetActorLocation`)) "AlwaysSpawn" "MultiplyWithRoot" null null)
          (break))))))

(fn `UserConstructionScript`
  (bind _output_get (set `self.As BPC Outfit Controller` (`self.GetComponentByClass` "/Game/Broquere/Zombie/Master/BPC_OutfitController_Testing.BPC_OutfitController_Testing_C")))
  (`/Game/Broquere/Zombie/Master/BPC_OutfitController_Testing.RandomizeSelected` _output_get null))

(fn `ZombieCantStayInPlace`
  (if (< (`self.DelayToDeath`) 10)
    (if (not (> (`KismetMathLibrary.VSizeXY` (`MovementComponent.Velocity` (`self.CharacterMovement`))) 50.0))
      (`/Engine/EditorBlueprintResources/StandardMacros.IncrementInt` (`self.DelayToDeath`))
      (else
        (set `self.DelayToDeath` 0)))
    (else
      (`GameplayStatics.ApplyDamage` self 99999999.0 null self)
      (`KismetSystemLibrary.K2_ClearAndInvalidateTimerHandle` (`self.Event_ZombieCantStayInPlace`)))))