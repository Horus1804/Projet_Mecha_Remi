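; Wave-based zombie spawner that reads zombie count and stats from DT_ZombiePerWave using the player's current wave.
; After a short delay at BeginPlay, a timer-chained HandleSpawn spawns batches at randomly picked spawn points until the count runs out.
; Each zombie receives a barricade reference, damage, health and score, and is set running.
; HandleWave advances the wave, restarts spawning and updates the HUD once no zombies remain.
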(event `HandleSpawn`
  (if (> (`self.ZombieCount`) 0)
    (for _ (range 3)
      (`self.SpawnZombies`)
      (`/Engine/EditorBlueprintResources/StandardMacros.DecrementInt` (`self.ZombieCount`)))
    (`KismetSystemLibrary.K2_SetTimerDelegate` (delegate `HandleSpawn`) 2.0)))

(event `SpawnWave`
  (bind _returnvalue (`|GetDataTableRow` "/Game/Broquere/DT_ZombiePerWave.DT_ZombiePerWave" (`KismetStringLibrary.Conv_StringToName` (`KismetStringLibrary.Conv_IntToString` (`/Game/Assets/Blueprint/Player/BP_Player.Wave` (`self.As BP Player`)))) :!label _label)
    (:`then`
      (bind _output_get (set `self.Out Row` _returnvalue))
      (set `self.ZombieCount` (- (`.NumberOfZombie_19_AC40A6DA4DCFF2B820BF779D7F437463` (break `/Game/Broquere/SwaveTable` _output_get)) 1))
      (`self.HandleSpawn`))
    (:`RowNotFound`
      (`KismetSystemLibrary.PrintString` "pas trouvé"))))

(event `self.ReceiveBeginPlay`
  (`self.GetSpawn`)
  (bind _asbp_player (cast `/Game/Assets/Blueprint/Player/BP_Player` (`GameplayStatics.GetPlayerCharacter` 0)))
  (set `self.As BP Player` _asbp_player)
  (`KismetSystemLibrary.Delay` 2.0)
  (goto _label))

(event `SpawnZombies`
  (bind (_numberofzombie _ratioscore _damage _health) (break `/Game/Broquere/SwaveTable` (`self.Out Row`)))
  (bind (_outitem _outindex) (`KismetArrayLibrary.Array_Random` (`self.SpawnLocation`)))
  (set `self.Random Spawn Location` _outindex)
  (bind _returnvalue (`|SpawnActorFromClass` "/Game/Broquere/Zombie/Zombie_01/BP_Child_ZombieMaster_01.BP_Child_ZombieMaster_01_C" (`KismetMathLibrary.MakeTransform` _outitem) "AdjustIfPossibleButAlwaysSpawn" "MultiplyWithRoot" null self null))
  (bind _output_get (set `self.Zombie Ref` _returnvalue))
  (set `/Game/Broquere/AI/AIC_Zombie.RefBarricade` (`|GetArrayItem` (`self.RefBarricade`) (`self.Random Spawn Location`)) (`/Game/Broquere/Zombie/Master/BP_ZombieMaster.RefAIC Zombie` _output_get))
  (`/Engine/EditorBlueprintResources/StandardMacros.IncrementInt` (`self.NumberOfZombies`)
    (:`  `
      (bind _zombie_ref (`self.Zombie Ref`)
        (:`then`
          (set `/Game/Broquere/Zombie/Master/BP_ZombieMaster.AttackDamage` _damage _zombie_ref)
          (set `/Game/Broquere/Zombie/Master/BP_ZombieMaster.Health` _health _zombie_ref)
          (set `/Game/Broquere/Zombie/Master/BP_ZombieMaster.Score` _ratioscore _zombie_ref)
          (set `/Game/Broquere/Zombie/Master/BP_ZombieMaster.IsRunning` true _zombie_ref)
          (`KismetSystemLibrary.PrintString` (`KismetStringLibrary.Conv_DoubleToString` (`/Game/Broquere/Zombie/Master/BP_ZombieMaster.GetHealth` _output_get)))
          (`/Game/Broquere/Zombie/Master/BP_ZombieMaster.IsRunningZombi` _zombie_ref))
        (:`else`)))))

(event `HandleWave`
  (bind _as_bp_player (`self.As BP Player`))
  (bind _wave (`/Game/Assets/Blueprint/Player/BP_Player.Wave` _as_bp_player))
  ;[1 1 1] Handle wave
  (if (<= (`self.NumberOfZombies`) 0)
    (`/Engine/EditorBlueprintResources/StandardMacros.IncrementInt` _wave
      (:`  `
        (`self.SpawnWave`)
        (`/Game/CHARONNAT/UI/Blueprints/WBP_HUD.SetWavetext` (`/Game/Assets/Blueprint/Player/BP_Player.UI_HUD` _as_bp_player))
        (`KismetSystemLibrary.PrintText` (`|FormatText` "Wave : {A}" _wave))))))

(fn `GetSpawn`
  (`KismetArrayLibrary.Array_Clear` (`self.SpawnLocation`))
  (set `self.SpawnLocation` (`|MakeArray` (`SceneComponent.K2_GetComponentLocation` (`self.SpawnPoint`)) (`SceneComponent.K2_GetComponentLocation` (`self.SpawnPoint1`)) (`SceneComponent.K2_GetComponentLocation` (`self.SpawnPoint2`)) (`SceneComponent.K2_GetComponentLocation` (`self.SpawnPoint3`)))))

(fn `UserConstructionScript`)