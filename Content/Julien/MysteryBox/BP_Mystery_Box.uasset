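; Mystery box actor that sells the player a random weapon, showing a price widget when looked at up close.
; Interact checks money and plays an Actor Sequence, whose events cycle random meshes, spawn the weapon and start a close timer.
; Closing deducts the cost and destroys an untaken weapon.
; Overlap gates a looping look check using a distance-scaled dot product; older timer and Tick-based animation code remains, marked old.
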(event `self.ReceiveBeginPlay`
  ;[0.04798 1 0] New Code With Actor Sequence
  (set `self.New_Player_Money` 0)
  (bind _returnvalue (`KismetSystemLibrary.K2_SetTimer` null "Is looking" 0.1 true))
  (bind _output_get (set `self.PlayerLookTimer` _returnvalue))
  (`KismetSystemLibrary.K2_PauseTimerHandle` _output_get)
  (bind _returnvalue_2 (`|CreateWidget` "/Game/CHARONNAT/UI/Blueprints/WBP_Price.WBP_Price_C"))
  (set `self.UIref` _returnvalue_2))

(event `Weapon_Down_to_Up`
  (bind (_relativelocation_x _relativelocation_y _relativelocation_z) (`KismetMathLibrary.BreakVector` (`SceneComponent.RelativeLocation` (`self.Random_Weapon`))))
  ;[0.125 0.125 0.125] Old_Code
  ;;[1 0 0.009549] Weapon_Down_to_Up_Event
  (if (`self.Openning_Box`)
    (set `self.Random_Weapon_Initial_Location` _relativelocation_z)
    (`SceneComponent.K2_SetRelativeLocation` (`self.Random_Weapon`) (`KismetMathLibrary.MakeVector` 0.0 0.0 (`KismetMathLibrary.Lerp` (`self.Random_Weapon_Initial_Location`) (`self.Random_Weapon_New_Location`) (`self.Delta Seconds`))) false false)))

(event `self.ReceiveTick`
  (params (DeltaSeconds :type "Float (single-precision)"))
  ;[0.125 0.125 0.125] Old_Code
  ;;[0.5216 0.5216 0.5216] Tick_Event
)

(event `CloseBox`
  ;[0.04798 1 0] New Code With Actor Sequence
  ;;[0.08708 1 0] Anim (Box Opening, Random Anim, Box Closing)
  (bind _output_get (set `self.Player Ref` (stale `/Game/BlueprintCommun/BPI_Interact.Interact` PlayerRef) :!label _label))
  (if (>= (`/Game/Assets/Blueprint/Player/BP_Player.GetMoney` _output_get) (`self.MysteryMoney`))
    (if (and (`self.Openning_Box`) (`self.EndSequence`))
      (set `self.Openning_Box` false)
      (set `self.EndSequence` false)
      (bind _output_get_2 (set `self.New_Player_Money` (- (`/Game/Assets/Blueprint/Player/BP_Player.GetMoney` (`self.Player Ref`)) (`self.MysteryMoney`))))
      (`/Game/Assets/Blueprint/Player/BP_Player.SetMoney` (`self.Player Ref`) _output_get_2)
      (`SceneComponent.K2_SetRelativeRotation` :`self` (`self.MysteryBox_Cover`) :`bTeleport` true)
      (`SceneComponent.K2_SetRelativeLocation` (`self.Random_Weapon`) (0.0 0.0 30.0) false true)
      (`KismetSystemLibrary.K2_ClearAndInvalidateTimerHandle` (`self.TimerCloseBoxRef`))
      (bind _weaponref (`self.WeaponRef`)
        (:`then`
          (if (not (`/Game/Weapon/Blueprint/BP_WeaponParent.IsTaken` _weaponref))
            (`self.K2_DestroyActor` _weaponref)))
        (:`else`))
      (else
        (`ActorSequenceComponent.PlaySequence` (`self.ActorSequence`))))))

(event `/Game/BlueprintCommun/BPI_Interact.Interact`
  (params (PlayerRef :type "/Game/Assets/Blueprint/Player/BP_Player Object Reference"))
  ;[0.04798 1 0] New Code With Actor Sequence
  ;;[0.08708 1 0] Anim (Box Opening, Random Anim, Box Closing)
  (goto _label))

(event `Box_Openning`
  (bind _openning_box (`self.Openning_Box`))
  ;[0.125 0.125 0.125] Old_Code
  ;;[0 0.05153 1] Box Openning Event
  (set `self.Initial_Rotation` (`SceneComponent.RelativeRotation` (`self.MysteryBox_Cover`)))
  (`SceneComponent.K2_SetRelativeRotation` (`self.MysteryBox_Cover`) (`KismetMathLibrary.RInterpTo` (`self.Initial_Rotation`) (select `bool` _openning_box :`true` (struct :`Pitch` 90.0) :!type "Rotator Structure") (`self.Delta Seconds`) (select `bool` _openning_box :`false` 10.0 :`true` 2.0 :!type "Float (single-precision)")) false false))

(event `ResetMysteryBox`
  (params (Plr :type "/Game/Assets/Blueprint/Player/BP_Player Object Reference"))
  (bind _random_weapon (`self.Random_Weapon`))
  ;[0.125 0.125 0.125] Old_Code
  ;;[0 0 0] Reset_Mystery_Box
  (set `self.Openning_Box` false)
  (`StaticMeshComponent.SetStaticMesh` _random_weapon null)
  (`SceneComponent.K2_SetRelativeLocation` _random_weapon (0.0 0.0 0.0) false true)
  (set `self.IsFinish` false)
  (set `self.RandomStop` 0))

(event `Box_Interract`
  ;[0.125 0.125 0.125] Old_Code
  ;;[1 0.02061 0.868] Interact Box
  (if (and (not (`self.Openning_Box`)) (not (`self.IsFinish`)))
    (set `self.Openning_Box` true)
    (if (not (`KismetSystemLibrary.K2_IsValidTimerHandle` (`self.Event_RandomWeapons`)))
      (bind _returnvalue (`KismetSystemLibrary.K2_SetTimerDelegate` (`|CreateDelegate` :!event `SetRandomWeapons`) (`self.DelayLoopRandomizeWeapons`) true))
      (set `self.Event_RandomWeapons` _returnvalue)
      (`GameplayStatics.SpawnSoundAtLocation` "/Game/Julien/MysteryBox/Mystery_Box_Asset/Sound/SC_MisteryBox_Sound.SC_MisteryBox_Sound" (`SceneComponent.K2_GetComponentLocation` (`self.MysteryBox_Box`)) (struct) 1.0 1.0 0.0 null null))
    (elif (`self.IsFinish`)
      (`self.ResetMysteryBox` null))))

(event `self.Inner.OnComponentBeginOverlap`
  (params (OverlappedComponent :type "PrimitiveComponent Object Reference") (OtherActor :type "Actor Object Reference") (OtherComp :type "PrimitiveComponent Object Reference") (OtherBodyIndex :type Integer) (bFromSweep :type Boolean) (SweepResult :type "HitResult Structure (by ref)"))
  (if (not (`self.PlayerSetup?`))
    (bind _asbp_player (cast `/Game/Assets/Blueprint/Player/BP_Player` OtherActor))
    (set `self.As BP Player` _asbp_player)
    (set `self.PlayerSetup?` true)
    (`KismetSystemLibrary.K2_UnPauseTimerHandle` (`self.PlayerLookTimer`))
    (else
      (cast `/Game/Assets/Blueprint/Player/BP_Player` OtherActor)
      (`KismetSystemLibrary.K2_UnPauseTimerHandle` (`self.PlayerLookTimer`)))))

(event `SetRandomWeapons`
  (bind _randomstop (`self.RandomStop`))
  (bind _randomstop_2 (`self.RandomStop`))
  ;[0.125 0.125 0.125] Old_Code
  ;;[1 0.4973 0.7823] Animation Random Weapons
  (if (and (>= _randomstop_2 20) (< _randomstop_2 21))
    (`/Engine/EditorBlueprintResources/StandardMacros.IncrementInt` (`self.RandomStop`)
      (:`  `
        (bind _output_get (set `self.DelayLoopRandomizeWeapons` 0.25))
        (bind _returnvalue (`KismetSystemLibrary.K2_SetTimerDelegate` (`|CreateDelegate` :!event `SetRandomWeapons`) _output_get true))
        (set `self.Event_RandomWeapons` _returnvalue))))
  (if (and (>= _randomstop 25) (< _randomstop 26))
    (bind _output_get_2 (set `self.DelayLoopRandomizeWeapons` 0.4))
    (bind _returnvalue_2 (`KismetSystemLibrary.K2_SetTimerDelegate` (`|CreateDelegate` :!event `SetRandomWeapons`) _output_get_2 true))
    (set `self.Event_RandomWeapons` _returnvalue_2))
  (if (and (`self.Openning_Box`) (!= (`self.RandomStop`) 32))
    (`StaticMeshComponent.SetStaticMesh` (`self.Random_Weapon`) (`KismetArrayLibrary.Array_Random` (`self.Weapon_Array`)))
    (`/Engine/EditorBlueprintResources/StandardMacros.IncrementInt` (`self.RandomStop`))
    (else
      (set `self.IsFinish` true)
      (`KismetSystemLibrary.K2_ClearAndInvalidateTimerHandle` (`self.Event_RandomWeapons`)))))

(event `self.Inner.OnComponentEndOverlap`
  (params (OverlappedComponent :type "PrimitiveComponent Object Reference") (OtherActor :type "Actor Object Reference") (OtherComp :type "PrimitiveComponent Object Reference") (OtherBodyIndex :type Integer))
  (cast `/Game/Assets/Blueprint/Player/BP_Player` OtherActor)
  (bind _uiref (`self.UIref`)
    (:`then`
      (`Widget.RemoveFromParent` _uiref)
      (`KismetSystemLibrary.K2_PauseTimerHandle` (`self.PlayerLookTimer`)))
    (:`else`)))

(event `StartSequence`
  (params (BP_Mystery_Box0 :type "Actor Object Reference"))
  ;[0.07561 1 0] Event_Start_Sequence
  (set `self.Openning_Box` true))

(event `Anim_Random_Weapon`
  (params (Owner :type "Actor Object Reference"))
  ;[1 0.4469 0] Event_Anim_Random_Weapon
  (`StaticMeshComponent.SetStaticMesh` (`self.Random_Weapon`) (`KismetArrayLibrary.Array_Random` (`self.Weapon_Array`))))

(event `End_Anim_Random_Weapon`
  (params (Owner :type "Actor Object Reference"))
  ;[1 0 0] Event_End_Sequence
  (set `self.EndSequence` true)
  (`StaticMeshComponent.SetStaticMesh` (`self.Random_Weapon`) null)
  (bind _returnvalue (`|SpawnActorFromClass` (`KismetArrayLibrary.Array_Random` (`self.Weapon_Class`)) (`KismetMathLibrary.MakeTransform` (`SceneComponent.K2_GetComponentLocation` (`self.Random_Weapon`)) (`KismetMathLibrary.MakeRotator` (.roll (`self.K2_GetActorRotation`)) (.pitch (`self.K2_GetActorRotation`)) (+ (.yaw (`self.K2_GetActorRotation`)) 90.0))) "Undefined" "MultiplyWithRoot" null null))
  (set `self.WeaponRef` _returnvalue)
  (bind _returnvalue_2 (`KismetSystemLibrary.K2_SetTimerDelegate` (`|CreateDelegate` :!event `cLoseBox`) 3.0))
  (set `self.TimerCloseBoxRef` _returnvalue_2))

(fn `Is looking`
  (bind _arrow (`self.Arrow`))
  (bind _camera (`/Game/Assets/Blueprint/Player/BP_Player.Camera` (`self.As BP Player`)))
  (if (< (`KismetMathLibrary.Dot_VectorVector` (`SceneComponent.GetForwardVector` _camera) (`SceneComponent.GetForwardVector` _arrow)) (`KismetMathLibrary.Lerp` -0.5 -1.0 (/ (`KismetMathLibrary.Vector_Distance` (`SceneComponent.K2_GetComponentLocation` _camera) (`SceneComponent.K2_GetComponentLocation` _arrow)) 360.0)))
    (`/Engine/EditorBlueprintResources/StandardMacros.DoOnce` false :!label _label
      (:`Completed`
        (set `self.IsLooking` true)
        (bind _uiref (`self.UIref`)
          (:`then`
            (`UserWidget.AddToViewport` _uiref 0)
            (set `WidgetSwitcher.ActiveWidgetIndex` 1 (`/Game/CHARONNAT/UI/Blueprints/WBP_Price.WidgetSwitcher` _uiref))
            (goto _label_2 :!via `Reset`))
          (:`else`))))
    (else
      (`/Engine/EditorBlueprintResources/StandardMacros.DoOnce` false :!label _label_2
        (:`Completed`
          (set `self.IsLooking` false)
          (bind _uiref_2 (`self.UIref`)
            (:`then`
              (`Widget.RemoveFromParent` _uiref_2)
              (goto _label :!via `Reset`))
            (:`else`)))))))

(fn `UserConstructionScript`)