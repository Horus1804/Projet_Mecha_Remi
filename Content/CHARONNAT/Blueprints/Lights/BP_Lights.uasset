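; BP_Lights is a configurable lamp actor with a static mesh and a spotlight.
; The construction script sets mesh and light rotation from the lamp type, and intensity, color and material from the lamp color (off, white, red or green).
; Flickering lamps get a light function material chosen by flicker speed.
; On BeginPlay it spawns a neon sound at its location, with a different cue for flickering and steady lamps.
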(event `self.ReceiveBeginPlay`
  (bind _returnvalue (`self.K2_GetActorLocation`))
  (if (`self.IsFlickering`)
    (bind _returnvalue_2 (`GameplayStatics.SpawnSoundAtLocation` "/Game/CHARONNAT/SoundDesign/Sounds/Ambiance/Neon/A_033830_fxlm-neon-lights-flicker-bathroomwav-75200_Cue.A_033830_fxlm-neon-lights-flicker-bathroomwav-75200_Cue" _returnvalue (struct) 1.0 1.0 0.0 null null))
    (`AudioComponent.Play` _returnvalue_2 0.0)
    (else
      (bind _returnvalue_3 (`GameplayStatics.SpawnSoundAtLocation` "/Game/CHARONNAT/SoundDesign/Sounds/Ambiance/Neon/A_neonlight_highpitch-7058_Cue.A_neonlight_highpitch-7058_Cue" _returnvalue (struct) 1.0 1.0 0.0 null null))
      (`AudioComponent.Play` _returnvalue_3 0.0))))

(fn `UserConstructionScript`
  (bind _lamptype (`self.LampType`))
  (bind _spotlight (`self.SpotLight`))
  (bind _spotlight_2 (`self.SpotLight`))
  (`StaticMeshComponent.SetStaticMesh` (`self.StaticMesh`) (select `/Game/CHARONNAT/Blueprints/Lights/E_LampsType` _lamptype :`NewEnumerator0` "/Game/Hospital_Meshingun/Environment/Asset/Mesh/Props/SM_Lamp_02a.SM_Lamp_02a" :`NewEnumerator1` "/Game/Hospital_Meshingun/Environment/Asset/Mesh/Props/SM_Lamp_02b.SM_Lamp_02b" :!type "StaticMesh Object Reference"))
  (`SceneComponent.K2_SetRelativeRotation` (`self.SpotLight`) (select `/Game/CHARONNAT/Blueprints/Lights/E_LampsType` _lamptype :`NewEnumerator0` (struct :`Pitch` -90.0) :`NewEnumerator1` (struct :`Pitch` -40.0 :`Yaw` 180.0 :`Roll` -180.0) :!type "Rotator Structure") false false)
  (switch `/Game/CHARONNAT/Blueprints/Lights/E_LightColor` (`self.LampsColor`)
    (:`NewEnumerator0`
      (`LightComponent.SetIntensity` (`self.SpotLight`) 0.0)
      (`PrimitiveComponent.SetMaterial` (`self.StaticMesh`) 0 "/Game/Hospital_Meshingun/Environment/Asset/Material/props/MI_lamp_02a.MI_Lamp_02a"))
    (:`NewEnumerator1`
      (`LightComponent.SetIntensity` (`self.SpotLight`) (`self.Intensity`))
      (`PrimitiveComponent.SetMaterial` (`self.StaticMesh`) 0 "/Game/Hospital_Meshingun/Environment/Asset/Material/props/MI_lamp_02b.MI_Lamp_02b"))
    (:`NewEnumerator2`
      (`LightComponent.SetIntensity` _spotlight_2 (`self.Intensity`))
      (`LightComponent.SetLightColor` _spotlight_2 (struct :`R` 0.822917 :`A` 1.0) true)
      (`PrimitiveComponent.SetMaterial` (`self.StaticMesh`) 0 "/Game/Hospital_Meshingun/Environment/Asset/Material/props/MI_lamp_02c.MI_Lamp_02c"))
    (:`NewEnumerator3`
      (`LightComponent.SetIntensity` _spotlight (`self.Intensity`))
      (`LightComponent.SetLightColor` _spotlight (struct :`G` 0.822917 :`B` 0.071236 :`A` 1.0) true)
      (`PrimitiveComponent.SetMaterial` (`self.StaticMesh`) 0 "/Game/Hospital_Meshingun/Environment/Asset/Material/props/MI_lamp_02d.MI_Lamp_02d")))
  (if (`self.IsFlickering`)
    (`LightComponent.SetLightFunctionMaterial` (`self.SpotLight`) (select `byte` (`self.FlickerSpeed`) :`0` "/Game/Hospital_Meshingun/Master_Material/Flicker/Material/M_Flickering_LightFunction.M_Flickering_LightFunction" :`1` "/Game/Hospital_Meshingun/Master_Material/Flicker/Material/MI_Flickering_LightFunction_Fast.MI_Flickering_LightFunction_Fast" :`2` "/Game/Hospital_Meshingun/Master_Material/Flicker/Material/MI_Flickering_LightFunction_Slow.MI_Flickering_LightFunction_Slow" :!type "MaterialInterface Object Reference"))))