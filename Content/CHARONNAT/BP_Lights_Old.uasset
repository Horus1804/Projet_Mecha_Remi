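; BP_Lights_Old is a configurable lamp actor with a static mesh, two spotlights and an ambient sound.
; The Construction Script picks the mesh and visible spotlight from the lamp type, the material from the light state, and applies intensity to both spotlights.
; When flickering, the chosen spotlight gets a light function material matching the flicker speed.
; BeginPlay spawns a flicker or high-pitched neon sound at the actor's location.
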(event `self.ReceiveBeginPlay`
  (bind _returnvalue (`self.K2_GetActorLocation`))
  (if (`self.IsFlickering`)
    (bind _returnvalue_2 (`GameplayStatics.SpawnSoundAtLocation` "/Game/CHARONNAT/SoundDesign/Sounds/Ambiance/Neon/A_033830_fxlm-neon-lights-flicker-bathroomwav-75200_Cue.A_033830_fxlm-neon-lights-flicker-bathroomwav-75200_Cue" _returnvalue (struct) 1.0 1.0 0.0 null null))
    (`AudioComponent.Play` _returnvalue_2 0.0)
    (else
      (bind _returnvalue_3 (`GameplayStatics.SpawnSoundAtLocation` "/Game/CHARONNAT/SoundDesign/Sounds/Ambiance/Neon/A_neonlight_highpitch-7058_Cue.A_neonlight_highpitch-7058_Cue" _returnvalue (struct) 1.0 1.0 0.0 null null))
      (`AudioComponent.Play` _returnvalue_3 0.0))))

(fn `UserConstructionScript`
  (bind _lampstype (`self.LampsType`))
  (`PrimitiveComponent.SetMaterial` (`self.StaticMesh`) 0 (select `/Game/CHARONNAT/Enum/ETypeLight` (`self.ETypeLight`) :`NewEnumerator0` "/Game/Hospital_Meshingun/Environment/Asset/Material/props/MI_lamp_02a.MI_Lamp_02a" :`NewEnumerator1` "/Game/Hospital_Meshingun/Environment/Asset/Material/props/MI_lamp_02b.MI_Lamp_02b" :`NewEnumerator2` "/Game/Hospital_Meshingun/Environment/Asset/Material/props/MI_lamp_02c.MI_Lamp_02c" :`NewEnumerator3` "/Game/Hospital_Meshingun/Environment/Asset/Material/props/MI_lamp_02d.MI_Lamp_02d" :!type "MaterialInterface Object Reference"))
  (`LightComponent.SetIntensity` (`self.SpotLight_1`) (`self.Intensity`))
  (`LightComponent.SetIntensity` (`self.SpotLight_2`) (`self.Intensity`))
  (`StaticMeshComponent.SetStaticMesh` (`self.StaticMesh`) (select `byte` _lampstype :`0` "/Game/Hospital_Meshingun/Environment/Asset/Mesh/Props/SM_Lamp_02a.SM_Lamp_02a" :`1` "/Game/Hospital_Meshingun/Environment/Asset/Mesh/Props/SM_Lamp_02b.SM_Lamp_02b" :!type "StaticMesh Object Reference"))
  (`SceneComponent.SetVisibility` (select `byte` _lampstype :`0` (`self.SpotLight_1`) :`1` (`self.SpotLight_2`) :!type "SceneComponent Object Reference") true false)
  (if (`self.IsFlickering`)
    (`LightComponent.SetLightFunctionMaterial` (select `byte` (`self.LampsType`) :`0` (`self.SpotLight_1`) :`1` (`self.SpotLight_2`) :!type "LightComponent Object Reference") (select `byte` (`self.FlickerSpeed`) :`0` "/Game/Hospital_Meshingun/Master_Material/Flicker/Material/M_Flickering_LightFunction.M_Flickering_LightFunction" :`1` "/Game/Hospital_Meshingun/Master_Material/Flicker/Material/MI_Flickering_LightFunction_Fast.MI_Flickering_LightFunction_Fast" :`2` "/Game/Hospital_Meshingun/Master_Material/Flicker/Material/MI_Flickering_LightFunction_Slow.MI_Flickering_LightFunction_Slow" :!type "MaterialInterface Object Reference"))))