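; Grenade actor that explodes once when damaged or hit by a shot, and starts a fuse-style timer on BeginPlay.
; A sphere's overlap events maintain the list of actors inside the blast zone.
; The explosion hides the grenade, plays particles and sound, calls ExplodeZombie on zombies, and damages players lightly and other actors heavily.
; An IsExplode flag blocks repeat blasts, and a short follow-up timer starts after detonation.
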(event `self.ReceiveBeginPlay`
  ;[0.4861 1 0.8484] Play
  (`KismetSystemLibrary.K2_SetTimerDelegate` (`|CreateDelegate` :!event `Explode`) 5.0))

(event `DestroyGrenade`
  ;[0.9036 1 0.565] Destroy Grenade
  (`self.K2_DestroyActor`))

(event `self.ReceiveAnyDamage`
  (params (Damage :type "Float (single-precision)") (DamageType :type "DamageType Object Reference") (InstigatedBy :type "Controller Object Reference") (DamageCauser :type "Actor Object Reference"))
  ;[0.1763 1 0.5596] Can take Damage
  (`self.Explode`))

(event `/Game/Weapon/BPI_Shoot.ShootHit`
  (params (HitZone :type "PhysicalMaterial Object Reference") (HitLocation :type "Vector Structure") (Causer :type "Actor Object Reference") (BaseDamage :type "Float (double-precision)"))
  ;[0.1763 1 0.5596] Can take Damage
  (`self.Explode`))

(event `Explode`
  (bind _returnvalue (`self.K2_GetActorLocation`))
  ;[1 0 0.06809] Explode Grenade
  (if (not (`self.IsExplode`))
    (set `self.IsExplode` true)
    (`SceneComponent.SetHiddenInGame` (`self.Grenade`) true false)
    (`GameplayStatics.SpawnEmitterAtLocation` "/Game/CROUZIE/FXVarietyPack/Particles/P_ky_explosion.P_ky_explosion" _returnvalue)
    (`GameplayStatics.PlaySoundAtLocation` "/Game/Assets/Audio/Weapons/LowQuality/Grenade_Set/SC_Grenade_Explosion_1_Cue.SC_Grenade_Explosion_1_Cue" _returnvalue (struct) 1.0 1.0 0.0 "/Game/YI_ModularZombies/Sounds/Master/SA_Basic.SA_Basic" null null null)
    (`SceneComponent.SetHiddenInGame` (`self.Sphere`) true false)
    (`self.ApplyDamageToAllActor`)
    (`KismetSystemLibrary.K2_SetTimerDelegate` (`|CreateDelegate` :!event `DestroyGrenade`) 2.0)))

(event `ApplyDamageToAllActor`
  (bind _actortohit (`self.ActorToHit`))
  ;[1 0.2142 0.8881] Apply Damage To Actor In Zone
  (if (`KismetArrayLibrary.Array_IsNotEmpty` _actortohit)
    (for _array_element _actortohit
      (`/Engine/EditorBlueprintResources/StandardMacros.IsValid` _array_element
        (:`Is Valid`
          (bind _asbp_zombie_master (cast `/Game/Broquere/Zombie/Master/BP_ZombieMaster` _array_element)
            (:`then`
              (`/Game/Broquere/Zombie/Master/BP_ZombieMaster.ExplodeZombie` _asbp_zombie_master))
            (:`CastFailed`
              (bind _asbp_player (cast `/Game/Assets/Blueprint/Player/BP_Player` _array_element)
                (:`then`
                  (`GameplayStatics.ApplyDamage` _asbp_player 1.0 null self))
                (:`CastFailed`
                  (`GameplayStatics.ApplyDamage` _array_element 100.0 null self))))))))))

(event `self.Sphere.OnComponentBeginOverlap`
  (params (OverlappedComponent :type "PrimitiveComponent Object Reference") (OtherActor :type "Actor Object Reference") (OtherComp :type "PrimitiveComponent Object Reference") (OtherBodyIndex :type Integer) (bFromSweep :type Boolean) (SweepResult :type "HitResult Structure (by ref)"))
  ;[0 0.3136 1] Zone Enter & Exit
  (if (not (`self.IsExplode`))
    (`KismetArrayLibrary.Array_Add` (`self.ActorToHit`) OtherActor)))

(event `self.Sphere.OnComponentEndOverlap`
  (params (OverlappedComponent :type "PrimitiveComponent Object Reference") (OtherActor :type "Actor Object Reference") (OtherComp :type "PrimitiveComponent Object Reference") (OtherBodyIndex :type Integer))
  (bind _actortohit (`self.ActorToHit`))
  ;[0 0.3136 1] Zone Enter & Exit
  (`KismetArrayLibrary.Array_Remove` _actortohit (`KismetArrayLibrary.Array_Find` _actortohit OtherActor)))

(fn `UserConstructionScript`)