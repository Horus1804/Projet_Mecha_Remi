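; BP_BoxTesting is a configurable test trigger zone that applies one effect, chosen by TypeBox, on overlap.
; Effects kill or damage the overlapping actor, add or set BP_Player health or money, or spawn a zombie at the box when a player enters.
; ObjectCanUseTrigger filters overlaps against an exact-class exclusion list containing BP_Grenade.
; The construction script labels and colors the text by type, with VisibleBox controlling in-game visibility of box and text.
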(event `self.Box.OnComponentBeginOverlap`
  (params (OverlappedComponent :type "PrimitiveComponent Object Reference") (OtherActor :type "Actor Object Reference") (OtherComp :type "PrimitiveComponent Object Reference") (OtherBodyIndex :type Integer) (bFromSweep :type Boolean) (SweepResult :type "HitResult Structure (by ref)"))
  (bind _isgood (`self.ObjectCanUseTrigger` OtherActor))
  (if _isgood
    (switch `/Game/Assets/Blueprint/TestingBox/Enum/ETypeBoxSystem` (`self.TypeBox`)
      (:`NewEnumerator0`
        ;[1 0 0] KILL
        (`GameplayStatics.ApplyDamage` (`self.ActorHit`) 9999999.0 null self))
      (:`NewEnumerator3`
        ;[1 0.3506 0] Set Damage
        (`GameplayStatics.ApplyDamage` (`self.ActorHit`) (`self.SetDamage`) null self))
      (:`NewEnumerator1`
        ;[1 0 0.6641] Add Health
        (bind _asbp_player (cast `/Game/Assets/Blueprint/Player/BP_Player` (`self.ActorHit`)))
        (`/Game/Assets/Blueprint/Player/BP_Player.AddHealth` _asbp_player (`KismetMathLibrary.Round` (`self.AddHealth`))))
      (:`NewEnumerator2`
        ;[0 1 0.1544] Set Health
        (bind _asbp_player_2 (cast `/Game/Assets/Blueprint/Player/BP_Player` (`self.ActorHit`)))
        (`/Game/Assets/Blueprint/Player/BP_Player.SetHealth` _asbp_player_2 (`KismetMathLibrary.Round` (`self.SetHealth`))))
      (:`NewEnumerator4`
        ;[0.6702 1 0] Spawn Zombie
        (cast `/Game/Assets/Blueprint/Player/BP_Player` (`self.ActorHit`))
        (`|SpawnActorFromClass` "/Game/Broquere/Zombie/Zombie_01/BP_Child_ZombieMaster_01.BP_Child_ZombieMaster_01_C" (`KismetMathLibrary.MakeTransform` (`self.K2_GetActorLocation`)) "Undefined" "MultiplyWithRoot" null null null))
      (:`NewEnumerator5`
        ;[0 0.8115 1] Add Money
        (bind _asbp_player_3 (cast `/Game/Assets/Blueprint/Player/BP_Player` (`self.ActorHit`)))
        (`/Game/Assets/Blueprint/Player/BP_Player.AddMoney` _asbp_player_3 (`self.AddMoney`)))
      (:`NewEnumerator6`
        ;[0 0.3181 1] Set Money
        (bind _asbp_player_4 (cast `/Game/Assets/Blueprint/Player/BP_Player` (`self.ActorHit`)))
        (`/Game/Assets/Blueprint/Player/BP_Player.SetMoney` _asbp_player_4 (`self.SetMoney`))))))

(fn `ObjectCanUseTrigger`
  (params (ActorHit :type "Actor Object Reference"))
  (returns (isGood :type Boolean))
  (locals (LocalClassToNotUse :type "Array of Actor Class Reference") (LocalCurrentClassToHit :type "Actor Class Reference") (`IsGood?` :type Boolean :default true))
  (bind _output_get (set `self.ActorHit` ActorHit))
  (set `local.LocalCurrentClassToHit` (`GameplayStatics.GetObjectClass` _output_get))
  (bind _output_get_2 (set `local.LocalClassToNotUse` (`|MakeArray` "/Game/Assets/Blueprint/Weapons/Grenade/BP_Grenade.BP_Grenade_C" :!type "Actor Class Reference")))
  (for _array_element _output_get_2
    (if (== _array_element (`local.LocalCurrentClassToHit`))
      (set `local.IsGood?` false)
      (break)))
  (return (`local.IsGood?`)))

(fn `UserConstructionScript`
  (bind _returnvalue (select `bool` (`self.VisibleBox`) :`false` true))
  (`TextRenderComponent.K2_SetText` (`self.TextRender`) (select `/Game/Assets/Blueprint/TestingBox/Enum/ETypeBoxSystem` (`self.TypeBox`) :`NewEnumerator0` "Kill Zone" :`NewEnumerator3` "Damage Zone" :`NewEnumerator1` "Add Health Zone" :`NewEnumerator2` "Set Health Zone" :`NewEnumerator4` "Spawn Zombie Zone" :`NewEnumerator5` "Add Money Zone" :`NewEnumerator6` "Set Money Zone"))
  (`TextRenderComponent.SetTextRenderColor` (`self.TextRender`) (select `/Game/Assets/Blueprint/TestingBox/Enum/ETypeBoxSystem` (`self.TypeBox`) :`NewEnumerator0` (make `Color` 0 0 255) :`NewEnumerator3` (make `Color` 1 30 255) :`NewEnumerator1` (make `Color` 0 255) :`NewEnumerator2` (make `Color` 30 255) :`NewEnumerator4` (make `Color` 30 255 30) :`NewEnumerator5` (make `Color` 255 255) :`NewEnumerator6` (make `Color` 255 255 30)))
  (`SceneComponent.SetHiddenInGame` (`self.TextRender`) _returnvalue false)
  (`SceneComponent.SetHiddenInGame` (`self.Box`) _returnvalue false))